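; MyGameState is a game state Blueprint that runs an in-game clock.
; Tick passes delta time and TimeUnit through SetClockWork to update ClockWork and DayTick, then calls Clock.
; Clock derives a 24-hour value from ClockWork through chained divisions and stores it as GameTime's third element.
; Minutes and seconds stay zero, and the debug print repeats only the first element, so the hour never displays.
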(event EventBeginPlay)

(event EventTick
  (params (DeltaSeconds :type Float%20%28single-precision%29))
  (Variables|Default|SetClockWork (.ClockworkOut (CallFunction|SetClockWork DeltaSeconds (Variables|Default|GetTimeUnit) (Variables|Default|GetClockWork))))
  (Variables|Default|SetDayTick (.DayTick (CallFunction|SetClockWork DeltaSeconds (Variables|Default|GetTimeUnit) (Variables|Default|GetClockWork))))
  (CallFunction|Clock))

(fn ConstructionScript)

(fn Clock
  (Variables|Default|SetHours (Math|Float|Floor (.Remainder (Math|Float|Division(WholeandRemainder) (Math|Conversions|ToFloat(Integer) (.ReturnValue (Math|Float|Division(WholeandRemainder) (Math|Conversions|ToFloat(Integer) (.ReturnValue (Math|Float|Division(WholeandRemainder) (* (Variables|Default|GetClockWork) 3.6e+03) 6e+01))) 6e+01))) 24.0))))
  (Variables|Default|SetGameTime (Utilities|Array|MakeArray 0 0 (Variables|Default|GetHours)))
  (Development|PrintString (Utilities|String|BuildString(Integer) (Utilities|String|BuildString(Integer) (Utilities|String|ToString(Integer) (Utilities|Array|Get(acopy) (Variables|Default|GetGameTime))) "" (Utilities|Array|Get(acopy) (Variables|Default|GetGameTime))) "" (Utilities|Array|Get(acopy) (Variables|Default|GetGameTime)))))