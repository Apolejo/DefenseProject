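; CameraPawn is a helper pawn that clears fog of war around the player character's position.
; On BeginPlay it caches the Player_Blueprint and starts a looping ClearFog timer.
; Each ClearFog call moves the pawn to the player and line-traces along its camera's forward vector on the Camera channel.
; When the trace hits a FogOfWar_BP, it passes the collision UV to DrawSubtract to erase fog there.
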(event Custom|ClearFog
  (bind _camera (Variables|Default|GetCamera))
  (bind _returnvalue (Transformation|GetWorldLocation _camera))
  (Transformation|SetActorLocation (Transformation|GetActorLocation (Variables|Default|GetPlayer_Ref)) false false)
  (bind (_outhit _returnvalue_2) (Collision|LineTraceByChannel _returnvalue (+ (* (Math|Vector|GetForwardVector (Variables|Default|GetCamera)) 1e+06) _returnvalue) "TraceTypeQuery2" true 0 "None"))
  (if _returnvalue_2
    (Utilities|IsValid (.HitActor (Collision|BreakHitResult _outhit))
      (:Is%20Valid
        (bind _asfog_of_war_bp (Utilities|Casting|CastToFogOfWar_BP (.HitActor (Collision|BreakHitResult _outhit))))
        (Default|DrawSubtract _asfog_of_war_bp (.UV (Class|GameplayStatics|FindCollisionUV _outhit)))))))

(event EventBeginPlay
  (bind _asplayer_blueprint (Utilities|Casting|CastToPlayer_Blueprint (Game|GetPlayerCharacter 0)))
  (Variables|Default|SetPlayer_Ref _asplayer_blueprint)
  (Utilities|Time|SetTimerbyFunctionName 0 "ClearFog" 0.1 true))

(fn ConstructionScript)