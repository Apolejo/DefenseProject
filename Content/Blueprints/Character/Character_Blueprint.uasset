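; Player character Blueprint for a layered 2D flipbook character that walks in four directions on the X/Y plane via movement input axes.
; Each Tick reads input and falling state, then AnimationStateMachine picks walk or idle states, prioritizing left, right, up, then down.
; Matching flipbooks drive the body sprite plus legs, helmet, chest, hands and arms layers.
; IdleDirection records last facing, but every idle branch selects the same Idle state.
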(event Custom|UpdateAnimation
  (bind (_isfalling _ismoving _moveleft _moveright _moveup _movedown) (CallFunction|GetDataOfMovement))
  (Utilities|IdleDirection
    (:GivesBoolWhoSaysDirection
      (bind (_outputmainflipbook _outputlegsflipbook _outputhelmetflipbook _outputchestflipbook _outputhandsflipbook _outputarmsflipbook) (CallFunction|AnimationStateMachine _isfalling _ismoving _moveleft _moveright _moveup _movedown))
      (Sprite|SetFlipbook (Variables|Default|GetSprite) _outputmainflipbook)
      (Utilities|AssetsFlipbook _outputlegsflipbook _outputhelmetflipbook _outputchestflipbook _outputhandsflipbook _outputarmsflipbook))))

(event EventBeginPlay
  (Class|ActorComponent|SetIsReplicated (Variables|Default|GetSprite) false))

(event EventTick
  (params (DeltaSeconds :type Float%20%28single-precision%29))
  (CallFunction|UpdateAnimation))

(event Input|AxisEvents|InputAxisMovementUpDown
  (params (AxisValue :type Float%20%28single-precision%29))
  ;[1 1 1] 2dMovement
  (Math|Float|CompareFloat AxisValue 0.0
    (:>
      (Variables|Movement|SetbIsMovingUp true))
    (:<
      (Variables|Movement|SetbIsMovingUp false)))
  (Pawn|Input|AddMovementInput "0.000000,1.000000, 0" AxisValue false))

(event Input|AxisEvents|InputAxisMovementRightLeft
  (params (AxisValue :type Float%20%28single-precision%29))
  ;[1 1 1] 2dMovement
  (Math|Float|CompareFloat AxisValue 0.0
    (:>
      (Variables|Movement|SetbIsMovingRight false))
    (:<
      (Variables|Movement|SetbIsMovingRight true)))
  (Pawn|Input|AddMovementInput "1.000000, 0, 0" AxisValue false))

(fn ConstructionScript)

(fn AnimationStateMachine
  (params (isFalling :type Boolean) (isMoving :type Boolean) (MoveLeft :type Boolean) (MoveRight :type Boolean) (MoveUp :type Boolean) (MoveDown :type Boolean))
  (|CollectData isFalling isMoving MoveLeft MoveRight MoveUp MoveDown)
  (if (not (LocalVariables|GetbLIsFalling?))
    (if (LocalVariables|GetbLIsMoving?)
      (if (LocalVariables|GetbLIsMoveLeft)
        (LocalVariables|SetAnimationState "NewEnumerator1")
        (LocalVariables|SetAnimationState_Legs "NewEnumerator1")
        (LocalVariables|SetAnimationState_Hands "NewEnumerator1")
        (LocalVariables|SetAnimationState_Arms "NewEnumerator1")
        (LocalVariables|SetAnimationState_Helmet "NewEnumerator1")
        (LocalVariables|SetAnimationState_Chest "NewEnumerator1")
        (return (Utilities|Select :Index (LocalVariables|GetAnimationState) :NewEnumerator0 (Variables|PlayerFlipbook|GetIdleFlipbook) :NewEnumerator1 (Variables|Player_Flipbook|GetFlipbook_WalkLeft) :NewEnumerator2 (Variables|Player_Flipbook|GetFlipbook_WalkRight) :NewEnumerator3 (Variables|Player_Flipbook|GetFlipbook_WalkUp) :NewEnumerator4 (Variables|Player_Flipbook|GetFlipbook_WalkDown)) (Utilities|Select :Index (LocalVariables|GetAnimationState_Legs) :NewEnumerator0 (Variables|LegsFlipbook|GetFB_Legs_IdleDown) :NewEnumerator1 (Variables|LegsFlipbook|GetFB_Legs_WalkLeft) :NewEnumerator2 (Variables|LegsFlipbook|GetFB_Legs_WalkRight) :NewEnumerator3 (Variables|LegsFlipbook|GetFB_Legs_WalkUp) :NewEnumerator4 (Variables|LegsFlipbook|GetFB_Legs_WalkDown)) (Utilities|Select :Index (LocalVariables|GetAnimationState_Helmet) :NewEnumerator0 (Variables|HelmetFlipbooks|GetFB_Helmet_IdleDown) :NewEnumerator1 (Variables|HelmetFlipbooks|GetFB_Helmet_WalkLeft) :NewEnumerator2 (Variables|HelmetFlipbooks|GetFB_Helmet_WalkRight) :NewEnumerator3 (Variables|HelmetFlipbooks|GetFB_Helmet_WalkUp) :NewEnumerator4 (Variables|HelmetFlipbooks|GetFB_Helmet_WalkDown)) (Utilities|Select :Index (LocalVariables|GetAnimationState_Chest) :NewEnumerator0 (Variables|ChestFlipbook|GetFB_Chest_IdleDown) :NewEnumerator1 (Variables|ChestFlipbook|GetFB_Chest_WalkLeft) :NewEnumerator2 (Variables|ChestFlipbook|GetFB_Chest_WalkRight) :NewEnumerator3 (Variables|ChestFlipbook|GetFB_Chest_WalkUp) :NewEnumerator4 (Variables|ChestFlipbook|GetFB_Chest_WalkDown)) (Utilities|Select :Index (LocalVariables|GetAnimationState_Hands) :NewEnumerator0 (Variables|HandsFlipbook|GetFB_Hands_IdleDown) :NewEnumerator1 (Variables|HandsFlipbook|GetFB_Hands_WalkLeft) :NewEnumerator2 (Variables|HandsFlipbook|GetFB_Hands_WalkRight) :NewEnumerator3 (Variables|HandsFlipbook|GetFB_Hands_WalkUp) :NewEnumerator4 (Variables|HandsFlipbook|GetFB_Hands_WalkDown)) (Utilities|Select :Index (LocalVariables|GetAnimationState_Arms) :NewEnumerator0 (Variables|ArmsFlipbook|GetFB_Arms_IdleDown) :NewEnumerator1 (Variables|ArmsFlipbook|GetFB_Arms_WalkLeft) :NewEnumerator2 (Variables|ArmsFlipbook|GetFB_Arms_WalkRight) :NewEnumerator3 (Variables|ArmsFlipbook|GetFB_Arms_WalkUp) :NewEnumerator4 (Variables|ArmsFlipbook|GetFB_Arms_WalkDown)))
        (elif (LocalVariables|GetbLMoveRight)
          (LocalVariables|SetAnimationState "NewEnumerator2")
          (LocalVariables|SetAnimationState_Legs "NewEnumerator2")
          (LocalVariables|SetAnimationState_Hands "NewEnumerator2")
          (LocalVariables|SetAnimationState_Arms "NewEnumerator2")
          (LocalVariables|SetAnimationState_Helmet "NewEnumerator2")
          (LocalVariables|SetAnimationState_Chest "NewEnumerator2")
          (return (Utilities|Select :Index (LocalVariables|GetAnimationState) :NewEnumerator0 (Variables|PlayerFlipbook|GetIdleFlipbook) :NewEnumerator1 (Variables|Player_Flipbook|GetFlipbook_WalkLeft) :NewEnumerator2 (Variables|Player_Flipbook|GetFlipbook_WalkRight) :NewEnumerator3 (Variables|Player_Flipbook|GetFlipbook_WalkUp) :NewEnumerator4 (Variables|Player_Flipbook|GetFlipbook_WalkDown)) (Utilities|Select :Index (LocalVariables|GetAnimationState_Legs) :NewEnumerator0 (Variables|LegsFlipbook|GetFB_Legs_IdleDown) :NewEnumerator1 (Variables|LegsFlipbook|GetFB_Legs_WalkLeft) :NewEnumerator2 (Variables|LegsFlipbook|GetFB_Legs_WalkRight) :NewEnumerator3 (Variables|LegsFlipbook|GetFB_Legs_WalkUp) :NewEnumerator4 (Variables|LegsFlipbook|GetFB_Legs_WalkDown)) (Utilities|Select :Index (LocalVariables|GetAnimationState_Helmet) :NewEnumerator0 (Variables|HelmetFlipbooks|GetFB_Helmet_IdleDown) :NewEnumerator1 (Variables|HelmetFlipbooks|GetFB_Helmet_WalkLeft) :NewEnumerator2 (Variables|HelmetFlipbooks|GetFB_Helmet_WalkRight) :NewEnumerator3 (Variables|HelmetFlipbooks|GetFB_Helmet_WalkUp) :NewEnumerator4 (Variables|HelmetFlipbooks|GetFB_Helmet_WalkDown)) (Utilities|Select :Index (LocalVariables|GetAnimationState_Chest) :NewEnumerator0 (Variables|ChestFlipbook|GetFB_Chest_IdleDown) :NewEnumerator1 (Variables|ChestFlipbook|GetFB_Chest_WalkLeft) :NewEnumerator2 (Variables|ChestFlipbook|GetFB_Chest_WalkRight) :NewEnumerator3 (Variables|ChestFlipbook|GetFB_Chest_WalkUp) :NewEnumerator4 (Variables|ChestFlipbook|GetFB_Chest_WalkDown)) (Utilities|Select :Index (LocalVariables|GetAnimationState_Hands) :NewEnumerator0 (Variables|HandsFlipbook|GetFB_Hands_IdleDown) :NewEnumerator1 (Variables|HandsFlipbook|GetFB_Hands_WalkLeft) :NewEnumerator2 (Variables|HandsFlipbook|GetFB_Hands_WalkRight) :NewEnumerator3 (Variables|HandsFlipbook|GetFB_Hands_WalkUp) :NewEnumerator4 (Variables|HandsFlipbook|GetFB_Hands_WalkDown)) (Utilities|Select :Index (LocalVariables|GetAnimationState_Arms) :NewEnumerator0 (Variables|ArmsFlipbook|GetFB_Arms_IdleDown) :NewEnumerator1 (Variables|ArmsFlipbook|GetFB_Arms_WalkLeft) :NewEnumerator2 (Variables|ArmsFlipbook|GetFB_Arms_WalkRight) :NewEnumerator3 (Variables|ArmsFlipbook|GetFB_Arms_WalkUp) :NewEnumerator4 (Variables|ArmsFlipbook|GetFB_Arms_WalkDown)))
          (elif (LocalVariables|GetbLMoveUp)
            (LocalVariables|SetAnimationState "NewEnumerator3")
            (LocalVariables|SetAnimationState_Legs "NewEnumerator3")
            (LocalVariables|SetAnimationState_Hands "NewEnumerator3")
            (LocalVariables|SetAnimationState_Arms "NewEnumerator3")
            (LocalVariables|SetAnimationState_Helmet "NewEnumerator3")
            (LocalVariables|SetAnimationState_Chest "NewEnumerator3")
            (return (Utilities|Select :Index (LocalVariables|GetAnimationState) :NewEnumerator0 (Variables|PlayerFlipbook|GetIdleFlipbook) :NewEnumerator1 (Variables|Player_Flipbook|GetFlipbook_WalkLeft) :NewEnumerator2 (Variables|Player_Flipbook|GetFlipbook_WalkRight) :NewEnumerator3 (Variables|Player_Flipbook|GetFlipbook_WalkUp) :NewEnumerator4 (Variables|Player_Flipbook|GetFlipbook_WalkDown)) (Utilities|Select :Index (LocalVariables|GetAnimationState_Legs) :NewEnumerator0 (Variables|LegsFlipbook|GetFB_Legs_IdleDown) :NewEnumerator1 (Variables|LegsFlipbook|GetFB_Legs_WalkLeft) :NewEnumerator2 (Variables|LegsFlipbook|GetFB_Legs_WalkRight) :NewEnumerator3 (Variables|LegsFlipbook|GetFB_Legs_WalkUp) :NewEnumerator4 (Variables|LegsFlipbook|GetFB_Legs_WalkDown)) (Utilities|Select :Index (LocalVariables|GetAnimationState_Helmet) :NewEnumerator0 (Variables|HelmetFlipbooks|GetFB_Helmet_IdleDown) :NewEnumerator1 (Variables|HelmetFlipbooks|GetFB_Helmet_WalkLeft) :NewEnumerator2 (Variables|HelmetFlipbooks|GetFB_Helmet_WalkRight) :NewEnumerator3 (Variables|HelmetFlipbooks|GetFB_Helmet_WalkUp) :NewEnumerator4 (Variables|HelmetFlipbooks|GetFB_Helmet_WalkDown)) (Utilities|Select :Index (LocalVariables|GetAnimationState_Chest) :NewEnumerator0 (Variables|ChestFlipbook|GetFB_Chest_IdleDown) :NewEnumerator1 (Variables|ChestFlipbook|GetFB_Chest_WalkLeft) :NewEnumerator2 (Variables|ChestFlipbook|GetFB_Chest_WalkRight) :NewEnumerator3 (Variables|ChestFlipbook|GetFB_Chest_WalkUp) :NewEnumerator4 (Variables|ChestFlipbook|GetFB_Chest_WalkDown)) (Utilities|Select :Index (LocalVariables|GetAnimationState_Hands) :NewEnumerator0 (Variables|HandsFlipbook|GetFB_Hands_IdleDown) :NewEnumerator1 (Variables|HandsFlipbook|GetFB_Hands_WalkLeft) :NewEnumerator2 (Variables|HandsFlipbook|GetFB_Hands_WalkRight) :NewEnumerator3 (Variables|HandsFlipbook|GetFB_Hands_WalkUp) :NewEnumerator4 (Variables|HandsFlipbook|GetFB_Hands_WalkDown)) (Utilities|Select :Index (LocalVariables|GetAnimationState_Arms) :NewEnumerator0 (Variables|ArmsFlipbook|GetFB_Arms_IdleDown) :NewEnumerator1 (Variables|ArmsFlipbook|GetFB_Arms_WalkLeft) :NewEnumerator2 (Variables|ArmsFlipbook|GetFB_Arms_WalkRight) :NewEnumerator3 (Variables|ArmsFlipbook|GetFB_Arms_WalkUp) :NewEnumerator4 (Variables|ArmsFlipbook|GetFB_Arms_WalkDown)))
            (elif (LocalVariables|GetLMoveDown)
              (LocalVariables|SetAnimationState "NewEnumerator4")
              (LocalVariables|SetAnimationState_Legs "NewEnumerator4")
              (LocalVariables|SetAnimationState_Hands "NewEnumerator4")
              (LocalVariables|SetAnimationState_Arms "NewEnumerator4")
              (LocalVariables|SetAnimationState_Helmet "NewEnumerator4")
              (LocalVariables|SetAnimationState_Chest "NewEnumerator4")
              (return (Utilities|Select :Index (LocalVariables|GetAnimationState) :NewEnumerator0 (Variables|PlayerFlipbook|GetIdleFlipbook) :NewEnumerator1 (Variables|Player_Flipbook|GetFlipbook_WalkLeft) :NewEnumerator2 (Variables|Player_Flipbook|GetFlipbook_WalkRight) :NewEnumerator3 (Variables|Player_Flipbook|GetFlipbook_WalkUp) :NewEnumerator4 (Variables|Player_Flipbook|GetFlipbook_WalkDown)) (Utilities|Select :Index (LocalVariables|GetAnimationState_Legs) :NewEnumerator0 (Variables|LegsFlipbook|GetFB_Legs_IdleDown) :NewEnumerator1 (Variables|LegsFlipbook|GetFB_Legs_WalkLeft) :NewEnumerator2 (Variables|LegsFlipbook|GetFB_Legs_WalkRight) :NewEnumerator3 (Variables|LegsFlipbook|GetFB_Legs_WalkUp) :NewEnumerator4 (Variables|LegsFlipbook|GetFB_Legs_WalkDown)) (Utilities|Select :Index (LocalVariables|GetAnimationState_Helmet) :NewEnumerator0 (Variables|HelmetFlipbooks|GetFB_Helmet_IdleDown) :NewEnumerator1 (Variables|HelmetFlipbooks|GetFB_Helmet_WalkLeft) :NewEnumerator2 (Variables|HelmetFlipbooks|GetFB_Helmet_WalkRight) :NewEnumerator3 (Variables|HelmetFlipbooks|GetFB_Helmet_WalkUp) :NewEnumerator4 (Variables|HelmetFlipbooks|GetFB_Helmet_WalkDown)) (Utilities|Select :Index (LocalVariables|GetAnimationState_Chest) :NewEnumerator0 (Variables|ChestFlipbook|GetFB_Chest_IdleDown) :NewEnumerator1 (Variables|ChestFlipbook|GetFB_Chest_WalkLeft) :NewEnumerator2 (Variables|ChestFlipbook|GetFB_Chest_WalkRight) :NewEnumerator3 (Variables|ChestFlipbook|GetFB_Chest_WalkUp) :NewEnumerator4 (Variables|ChestFlipbook|GetFB_Chest_WalkDown)) (Utilities|Select :Index (LocalVariables|GetAnimationState_Hands) :NewEnumerator0 (Variables|HandsFlipbook|GetFB_Hands_IdleDown) :NewEnumerator1 (Variables|HandsFlipbook|GetFB_Hands_WalkLeft) :NewEnumerator2 (Variables|HandsFlipbook|GetFB_Hands_WalkRight) :NewEnumerator3 (Variables|HandsFlipbook|GetFB_Hands_WalkUp) :NewEnumerator4 (Variables|HandsFlipbook|GetFB_Hands_WalkDown)) (Utilities|Select :Index (LocalVariables|GetAnimationState_Arms) :NewEnumerator0 (Variables|ArmsFlipbook|GetFB_Arms_IdleDown) :NewEnumerator1 (Variables|ArmsFlipbook|GetFB_Arms_WalkLeft) :NewEnumerator2 (Variables|ArmsFlipbook|GetFB_Arms_WalkRight) :NewEnumerator3 (Variables|ArmsFlipbook|GetFB_Arms_WalkUp) :NewEnumerator4 (Variables|ArmsFlipbook|GetFB_Arms_WalkDown)))))))
      (else
        (if (Variables|Default|GetWasMovingUp)
          (LocalVariables|SetAnimationState "NewEnumerator0")
          (LocalVariables|SetAnimationState_Legs "NewEnumerator0")
          (LocalVariables|SetAnimationState_Hands "NewEnumerator0")
          (LocalVariables|SetAnimationState_Arms "NewEnumerator0")
          (LocalVariables|SetAnimationState_Helmet "NewEnumerator0")
          (LocalVariables|SetAnimationState_Chest "NewEnumerator0")
          (elif (Variables|Default|GetWasMovingDown)
            (LocalVariables|SetAnimationState "NewEnumerator0")
            (LocalVariables|SetAnimationState_Legs "NewEnumerator0")
            (LocalVariables|SetAnimationState_Hands "NewEnumerator0")
            (LocalVariables|SetAnimationState_Arms "NewEnumerator0")
            (LocalVariables|SetAnimationState_Helmet "NewEnumerator0")
            (LocalVariables|SetAnimationState_Chest "NewEnumerator0")
            (elif (Variables|Default|GetWasMovingLeft)
              (LocalVariables|SetAnimationState "NewEnumerator0")
              (LocalVariables|SetAnimationState_Legs "NewEnumerator0")
              (LocalVariables|SetAnimationState_Hands "NewEnumerator0")
              (LocalVariables|SetAnimationState_Arms "NewEnumerator0")
              (LocalVariables|SetAnimationState_Helmet "NewEnumerator0")
              (LocalVariables|SetAnimationState_Chest "NewEnumerator0")
              (elif (Variables|Default|GetWasMovingRight)
                (LocalVariables|SetAnimationState "NewEnumerator0")
                (LocalVariables|SetAnimationState_Legs "NewEnumerator0")
                (LocalVariables|SetAnimationState_Hands "NewEnumerator0")
                (LocalVariables|SetAnimationState_Arms "NewEnumerator0")
                (LocalVariables|SetAnimationState_Helmet "NewEnumerator0")
                (LocalVariables|SetAnimationState_Chest "NewEnumerator0")
                (else
                  (LocalVariables|SetAnimationState "NewEnumerator0")
                  (LocalVariables|SetAnimationState_Legs "NewEnumerator0")
                  (LocalVariables|SetAnimationState_Hands "NewEnumerator0")
                  (LocalVariables|SetAnimationState_Arms "NewEnumerator0")
                  (LocalVariables|SetAnimationState_Helmet "NewEnumerator0")
                  (LocalVariables|SetAnimationState_Chest "NewEnumerator0"))))))
        (return (Utilities|Select :Index (LocalVariables|GetAnimationState) :NewEnumerator0 (Variables|PlayerFlipbook|GetIdleFlipbook) :NewEnumerator1 (Variables|Player_Flipbook|GetFlipbook_WalkLeft) :NewEnumerator2 (Variables|Player_Flipbook|GetFlipbook_WalkRight) :NewEnumerator3 (Variables|Player_Flipbook|GetFlipbook_WalkUp) :NewEnumerator4 (Variables|Player_Flipbook|GetFlipbook_WalkDown)) (Utilities|Select :Index (LocalVariables|GetAnimationState_Legs) :NewEnumerator0 (Variables|LegsFlipbook|GetFB_Legs_IdleDown) :NewEnumerator1 (Variables|LegsFlipbook|GetFB_Legs_WalkLeft) :NewEnumerator2 (Variables|LegsFlipbook|GetFB_Legs_WalkRight) :NewEnumerator3 (Variables|LegsFlipbook|GetFB_Legs_WalkUp) :NewEnumerator4 (Variables|LegsFlipbook|GetFB_Legs_WalkDown)) (Utilities|Select :Index (LocalVariables|GetAnimationState_Helmet) :NewEnumerator0 (Variables|HelmetFlipbooks|GetFB_Helmet_IdleDown) :NewEnumerator1 (Variables|HelmetFlipbooks|GetFB_Helmet_WalkLeft) :NewEnumerator2 (Variables|HelmetFlipbooks|GetFB_Helmet_WalkRight) :NewEnumerator3 (Variables|HelmetFlipbooks|GetFB_Helmet_WalkUp) :NewEnumerator4 (Variables|HelmetFlipbooks|GetFB_Helmet_WalkDown)) (Utilities|Select :Index (LocalVariables|GetAnimationState_Chest) :NewEnumerator0 (Variables|ChestFlipbook|GetFB_Chest_IdleDown) :NewEnumerator1 (Variables|ChestFlipbook|GetFB_Chest_WalkLeft) :NewEnumerator2 (Variables|ChestFlipbook|GetFB_Chest_WalkRight) :NewEnumerator3 (Variables|ChestFlipbook|GetFB_Chest_WalkUp) :NewEnumerator4 (Variables|ChestFlipbook|GetFB_Chest_WalkDown)) (Utilities|Select :Index (LocalVariables|GetAnimationState_Hands) :NewEnumerator0 (Variables|HandsFlipbook|GetFB_Hands_IdleDown) :NewEnumerator1 (Variables|HandsFlipbook|GetFB_Hands_WalkLeft) :NewEnumerator2 (Variables|HandsFlipbook|GetFB_Hands_WalkRight) :NewEnumerator3 (Variables|HandsFlipbook|GetFB_Hands_WalkUp) :NewEnumerator4 (Variables|HandsFlipbook|GetFB_Hands_WalkDown)) (Utilities|Select :Index (LocalVariables|GetAnimationState_Arms) :NewEnumerator0 (Variables|ArmsFlipbook|GetFB_Arms_IdleDown) :NewEnumerator1 (Variables|ArmsFlipbook|GetFB_Arms_WalkLeft) :NewEnumerator2 (Variables|ArmsFlipbook|GetFB_Arms_WalkRight) :NewEnumerator3 (Variables|ArmsFlipbook|GetFB_Arms_WalkUp) :NewEnumerator4 (Variables|ArmsFlipbook|GetFB_Arms_WalkDown)))))))

(fn GetDataOfMovement
  (bind _returnvalue (Input|AxisValues|GetMovementUpDown))
  (bind _returnvalue_2 (Input|AxisValues|GetMovementRightLeft))
  (bind _output_get (Variables|Movement|SetbIsMovingDown (> _returnvalue 0.0)))
  (bind _output_get_2 (Variables|Movement|SetbIsMovingUp (< _returnvalue 0.0)))
  (bind _output_get_3 (Variables|Movement|SetbIsMoving? (not (and (== _returnvalue 0.0) (== _returnvalue_2 0.0)))))
  (bind _output_get_4 (Variables|Movement|SetbIsMovingRight (> _returnvalue_2 0.0)))
  (bind _output_get_5 (Variables|Movement|SetbIsMovingLeft (< _returnvalue_2 0.0)))
  (bind _output_get_6 (Variables|Movement|SetbIsFalling? (AI|Components|NavMovement|IsFalling (Variables|Character|GetCharacterMovement))))
  (return _output_get_6 _output_get_3 _output_get_5 _output_get_4 _output_get_2 _output_get))