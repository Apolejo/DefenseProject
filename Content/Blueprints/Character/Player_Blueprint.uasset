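; Player character for a 2D flipbook game with axis movement on the X/Y plane, layered equipment sprites and fog-of-war clearing.
; Each Tick, StateMachine reads the input axes to set directional walk flipbooks on body and armor layers, rotating the left-walk set 180° for the opposite direction.
; Tick also traces along the camera's forward vector, passing the hit's collision UV to FogOfWar_BP.DrawSubtract.
; A getter exposes vision range and angle.
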(event Custom|ClearFog
  (bind _camera (Variables|Default|GetCamera))
  (bind _returnvalue (Transformation|GetWorldLocation _camera))
  ;[1 1 1] ClearFog
  (bind (_outhit _returnvalue_2) (Collision|LineTraceByChannel _returnvalue (+ (* (Math|Vector|GetForwardVector _camera) 5e+03) _returnvalue) "TraceTypeQuery2" true 0 "None"))
  (if _returnvalue_2
    (Utilities|IsValid (.HitActor (Collision|BreakHitResult _outhit))
      (:Is%20Valid
        (bind _asfog_of_war_bp (Utilities|Casting|CastToFogOfWar_BP (.HitActor (Collision|BreakHitResult _outhit))))
        (Default|DrawSubtract _asfog_of_war_bp (.UV (Class|GameplayStatics|FindCollisionUV _outhit)))))))

(event EventBeginPlay
  (Class|ActorComponent|SetIsReplicated (Variables|Default|GetSprite) false))

(event Collision|EventActorBeginOverlap
  (params (OtherActor :type Actor%20Object%20Reference)))

(event EventTick
  (params (DeltaSeconds :type Float%20%28single-precision%29))
  (CallFunction|ClearFog)
  (if (not false)
    (CallFunction|StateMachine)))

(event Input|AxisEvents|InputAxisMovementUpDown
  (params (AxisValue :type Float%20%28single-precision%29))
  ;[1 1 1] 2dMovement
  (Math|Float|CompareFloat AxisValue 0.0
    (:>
      (Variables|Default|SetbIsMovingUp true))
    (:<
      (Variables|Default|SetbIsMovingUp false)))
  (Pawn|Input|AddMovementInput "0.000000,1.000000, 0" AxisValue false))

(event Input|AxisEvents|InputAxisMovementRightLeft
  (params (AxisValue :type Float%20%28single-precision%29))
  ;[1 1 1] 2dMovement
  (Math|Float|CompareFloat AxisValue 0.0
    (:>
      (Variables|Default|SetbIsMovingRight false))
    (:<
      (Variables|Default|SetbIsMovingRight true)))
  (Pawn|Input|AddMovementInput "1.000000, 0, 0" AxisValue false))

(fn ConstructionScript)

(fn StateMachine
  (bind _returnvalue (Input|AxisValues|GetMovementUpDown))
  (if (< _returnvalue 0.0)
    (Utilities|GoLeftorRight)
    (Sprite|SetFlipbook (Variables|Default|GetSprite) (Variables|Player_Flipbook|GetFlipbook_WalkUp))
    (Utilities|AssetsFlipbook (Variables|LegsFlipbook|GetFB_Legs_WalkUp) (Variables|HelmetFlipbooks|GetFB_Helmet_WalkUp) (Variables|ChestFlipbook|GetFB_Chest_WalkUp) (Variables|HandsFlipbook|GetFB_Hands_WalkUp) (Variables|ArmsFlipbook|GetFB_Arms_WalkUp))
    (elif (> _returnvalue 0.0)
      (Utilities|GoLeftorRight)
      (Sprite|SetFlipbook (Variables|Default|GetSprite) (Variables|Player_Flipbook|GetFlipbook_WalkDown))
      (Utilities|AssetsFlipbook (Variables|LegsFlipbook|GetFB_Legs_WalkDown) (Variables|HelmetFlipbooks|GetFB_Helmet_WalkDown) (Variables|ChestFlipbook|GetFB_Chest_WalkDown) (Variables|HandsFlipbook|GetFB_Hands_WalkDown) (Variables|ArmsFlipbook|GetFB_Arms_WalkDown))
      (elif (== _returnvalue 0.0)
        (Utilities|GoLeftorRight)))))

(fn RetrieveVisionRangeParameter
  (return (Variables|Default|GetVisionRange) (Variables|Default|GetVisionAngle)))