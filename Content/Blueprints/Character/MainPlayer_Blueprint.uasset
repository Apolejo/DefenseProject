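; Player Blueprint that handles interaction with nearby resource buildings, gated by an ImCloseToResource flag and a BuildingMasterREF reference.
; The action button collects from farms or fills water buildings, choosing by cast.
; PlacePlot passes an item ID to plant a farm or fuel a combustible energy building, printing a hint when out of range.
; UpgradeBuilding requests an upgrade check with a hard-coded test value.
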(event Custom|UpgradeBuilding
  ;[1 1 1] UpgradeTestPurposes
  (if (Variables|Default|GetImCloseToResource?)
    (Default|CheckUpgrade (Variables|Default|GetBuildingMasterREF) 200)))

(event Custom|PlacePlot
  (params (ItemId :type Integer))
  (bind _buildingmasterref (Variables|Default|GetBuildingMasterREF))
  (bind _buildingmasterref_2 (Variables|Default|GetBuildingMasterREF))
  (bind (_asfarm_building_bp _bsuccess) (Utilities|Casting|CastToFarmBuilding_BP _buildingmasterref_2))
  (bind (_asenergy_combustible_bp _bsuccess_2) (Utilities|Casting|CastToEnergyCombustible_BP _buildingmasterref))
  ;[1 1 1] ActivateBuildingResourceRecolection
  (if (Variables|Default|GetImCloseToResource?)
    (if _bsuccess
      (Default|PlantPlot _asfarm_building_bp ItemId)
      (elif _bsuccess_2
        (Default|MakingEnergy _asenergy_combustible_bp ItemId)))
    (else
      (Development|PrintString "Get closer"))))

(event EventBeginPlay
  (|CallParentFunction) ; This node is disabled and will not be called.\nDrag off pins to build functionality.
)

(event Collision|EventActorBeginOverlap
  (params (OtherActor :type Actor%20Object%20Reference)))

(event EventTick
  (params (DeltaSeconds :type Float%20%28single-precision%29))
  (|CallParentFunction DeltaSeconds) ; This node is disabled and will not be called.\nDrag off pins to build functionality.
)

(event Input|ActionEvents|InputActionActionButton
  (params (Key :type Key%20Structure))
  (bind _buildingmasterref (Variables|Default|GetBuildingMasterREF))
  (bind _buildingmasterref_2 (Variables|Default|GetBuildingMasterREF))
  (bind (_aswater_building_bp _bsuccess) (Utilities|Casting|CastToWaterBuilding_BP _buildingmasterref_2))
  (bind (_asfarm_building_bp _bsuccess_2) (Utilities|Casting|CastToFarmBuilding_BP _buildingmasterref))
  ;[1 1 1] Recolect Resources
  (:Pressed
    (if (Variables|Default|GetImCloseToResource?)
      (if _bsuccess_2
        (Default|ResourceCollected _asfarm_building_bp)
        (elif _bsuccess
          (Default|WaterFill _aswater_building_bp))))))

(fn ConstructionScript
  (|CallParentFunction))