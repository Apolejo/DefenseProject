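; Construction manager that runs timed building construction, tracking queued jobs in parallel proxy and config arrays.
; Queuing spawns the real building hidden plus a placeholder proxy that holds a reference to it, sized detection box, display mesh and build time.
; When a proxy reports completion, the manager removes both array entries, reveals the building, flags it completed and destroys the proxy.
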(event Custom|BindConstructionComplete
  (params (Proxy :type Construction%20Proxy%20BP%20Object%20Reference))
  (EventDispatchers|BindEventtoConstructionCompleted Proxy (EventDispatchers|CreateEvent :!event Custom|ConstructionCompleted)))

(event Custom|ConstructionCompleted
  (params (Proxy :type Construction%20Proxy%20BP%20Object%20Reference) (BuildingMaster_Ref :type Building%20Master%20BP%20Object%20Reference))
  (CallFunction|FinishConstruction Proxy BuildingMaster_Ref))

(fn ConstructionScript)

(fn QueueConstruction
  (params (ConstructionStruct :type Construction%20Struct%20Structure))
  (bind (_buildingclass _proxyclass _transform _displaymesh _buildingcollision _timerequired) (Utilities|Struct|BreakConstructionStruct ConstructionStruct))
  (bind _returnvalue (Game|SpawnActorfromClass _buildingclass _transform "AlwaysSpawn" 0 0 0))
  (bind _returnvalue_2 (Game|SpawnActorfromClass _proxyclass _transform "AlwaysSpawn" 0 _displaymesh _returnvalue 0))
  (Rendering|SetActorHiddenInGame _returnvalue true)
  (Components|Box|SetBoxExtent (Variables|/Game/Blueprints/Constructions/ConstructionProxy_BP.ConstructionProxy_BP_C|GetDetectZone _returnvalue_2) _buildingcollision true)
  (CallFunction|BindConstructionComplete _returnvalue_2)
  (Utilities|Array|Add (Variables|Default|GetProxies) _returnvalue_2)
  (Utilities|Array|Add (Variables|Default|GetQueue) ConstructionStruct)
  (Default|SetConstructionTime _returnvalue_2 _timerequired))

(fn FinishConstruction
  (params (Proxy :type Construction%20Proxy%20BP%20Object%20Reference) (BM_Ref :type Building%20Master%20BP%20Object%20Reference))
  (bind _proxies (Variables|Default|GetProxies))
  (bind _queue (Variables|Default|GetQueue))
  (bind _output_get (LocalVariables|SetIndex (Utilities|Array|FindItem _proxies Proxy)))
  (LocalVariables|SetConfig (Utilities|Array|Get(acopy) _queue _output_get))
  (Utilities|Array|RemoveIndex _queue (LocalVariables|GetIndex))
  (Utilities|Array|RemoveIndex _proxies (LocalVariables|GetIndex))
  (Rendering|SetActorHiddenInGame BM_Ref false)
  (Variables|/Game/Blueprints/Buldings/BuildingMaster_BP.BuildingMaster_BP_C|SetIsBuildingCompleted? BM_Ref true)
  (Actor|DestroyActor Proxy))