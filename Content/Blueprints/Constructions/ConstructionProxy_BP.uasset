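; Construction proxy actor that shows a ghost-material mesh of a pending building and builds it while the player stands nearby.
; DetectZone overlaps gate a Tick-driven timer that accumulates build time and updates a floating progress widget.
; When the construction time is reached, it fires ConstructionCompleted with itself and its building master, then destroys itself after a short delay.
; Cancelling from the widget returns resources through PlayerGameController and destroys both proxy and building master.
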(event OnComponentBeginOverlap(DetectZone)
  (params (OverlappedComponent :type Primitive%20Component%20Object%20Reference) (OtherActor :type Actor%20Object%20Reference) (OtherComp :type Primitive%20Component%20Object%20Reference) (OtherBodyIndex :type Integer) (bFromSweep :type Boolean) (SweepResult :type Hit%20Result%20Structure%20%28by%20ref%29))
  (if (.bSuccess (Utilities|Casting|CastToPlayer_Blueprint OtherActor))
    (Variables|Default|SetPlayerInside? true)))

(event OnComponentEndOverlap(DetectZone)
  (params (OverlappedComponent :type Primitive%20Component%20Object%20Reference) (OtherActor :type Actor%20Object%20Reference) (OtherComp :type Primitive%20Component%20Object%20Reference) (OtherBodyIndex :type Integer))
  (if (.bSuccess (Utilities|Casting|CastToPlayer_Blueprint OtherActor))
    (Variables|Default|SetPlayerInside? false)))

(event Custom|CancelConstructionAndReturnResources
  (CallFunction|ReturnResources)
  (Actor|DestroyActor)
  (Actor|DestroyActor (Variables|Default|GetBuildingMaster_Ref)))

(event EventBeginPlay
  (bind _output_get (Variables|Default|SetProgressWidget (.AsFloating%20Construction%20Widget (Utilities|Casting|CastToFloatingConstruction_Widget (UserInterface|GetUserWidgetObject (Variables|Default|GetBuildingLoading))))))
  (EventDispatchers|BindEventtoCancelConstruction _output_get (delegate Custom|CancelConstructionAndReturnResources)))

(event EventTick
  (params (DeltaSeconds :type Float%20%28single-precision%29))
  (bind _buildtimespent (Variables|Default|GetBuildTimeSpent))
  (bind _constructiontime (Variables|Default|GetConstructionTime))
  (Variables|Default|SetDelta DeltaSeconds)
  (if (not (Variables|Default|GetIsConstructionCompleted?))
    (if (Variables|Default|GetPlayerInside?)
      (CallFunction|DoBuild)
      (if (>= _buildtimespent _constructiontime)
        (Variables|Default|SetIsConstructionCompleted? true)
        (Default|CallConstructionCompleted self (Variables|Default|GetBuildingMaster_Ref))
        (Utilities|FlowControl|Delay 0.2)
        (Actor|DestroyActor)
        (else
          (Default|SetProgress (Variables|Default|GetProgressWidget) (/ _buildtimespent _constructiontime)))))))

(fn ConstructionScript
  (bind _staticmesh (Variables|Default|GetStaticMesh))
  (Components|StaticMesh|SetStaticMesh _staticmesh (Variables|Default|GetDisplayMesh))
  (Rendering|Material|SetMaterial _staticmesh 0 "/Game/Materials/BuildingMaterials/M_Ghost_Material.M_Ghost_Material"))

(fn SetConstructionTime
  (params (Time :type Float%20%28single-precision%29))
  (Variables|Default|SetConstructionTime (* Time 1.0))
  (return))

(fn DoBuild
  (bind _output_get (Variables|Default|SetClockWork (.ClockworkOut (CallFunction|SetClockWork (Variables|Default|GetDelta) (Variables|Default|GetTimeUnit) (Variables|Default|GetClockWork)))))
  (Variables|Default|SetBuildTimeSpent (* _output_get 1.0))
  (return))

(fn ReturnResources
  (bind _asplayer_game_controller (Utilities|Casting|CastToPlayerGameController (Game|GetPlayerController 0)))
  (Default|ReturnResource _asplayer_game_controller 1.0 (Variables|Default|GetBuildingMaster_Ref))
  (return))