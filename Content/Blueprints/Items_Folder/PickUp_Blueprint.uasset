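; Loot drop actor that scatters random human-part items and plasma around itself when it spawns.
; On BeginPlay it rolls a drop count and item IDs from cumulative chance arrays, then spawns each item's class from HumanParts_DataTable.
; Plasma appears as scattered mesh instances, and a player overlapping PickUpRange gains PlasmaDrop in their inventory.
; The actor destroys itself after that pickup, or right after spawning items if it holds no plasma.
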(event OnComponentBeginOverlap(PickUpRange)
  (params (OverlappedComponent :type Primitive%20Component%20Object%20Reference) (OtherActor :type Actor%20Object%20Reference) (OtherComp :type Primitive%20Component%20Object%20Reference) (OtherBodyIndex :type Integer) (bFromSweep :type Boolean) (SweepResult :type Hit%20Result%20Structure%20%28by%20ref%29))
  (bind _asmain_player_blueprint (Utilities|Casting|CastToMainPlayer_Blueprint OtherActor))
  (Variables|/Game/Blueprints/Character/MainPlayer_Blueprint.MainPlayer_Blueprint_C|SetPlayerInventory _asmain_player_blueprint (Utilities|Struct|MakePlayerInventory_Struct (.items100stacks (Variables|/Game/Blueprints/Character/MainPlayer_Blueprint.MainPlayer_Blueprint_C|GetPlayerInventory _asmain_player_blueprint)) (.items200stacks (Variables|/Game/Blueprints/Character/MainPlayer_Blueprint.MainPlayer_Blueprint_C|GetPlayerInventory _asmain_player_blueprint)) (+ (.plasma (Variables|/Game/Blueprints/Character/MainPlayer_Blueprint.MainPlayer_Blueprint_C|GetPlayerInventory _asmain_player_blueprint)) (Variables|Default|GetPlasmaDrop))))
  (Actor|DestroyActor))

(event EventBeginPlay
  (bind _returnvalue (Math|Random|RandomFloatinRange -25.0 25.0))
  (bind _returnvalue_2 (Math|Random|RandomFloatinRange -25.0 25.0))
  (bind _plasmadrop (Variables|Default|GetPlasmaDrop))
  (bind _returnvalue_3 (* _returnvalue 1.0))
  (bind _returnvalue_4 (* _returnvalue_2 1.0))
  (bind _returnvalue_5 (Math|Vector|MakeVector _returnvalue_4 _returnvalue_3 5.0))
  (bind _numberofdrops (CallFunction|RandomMaxDropwithChance (Variables|Default|GetDropMaxChance)))
  (for _index (range 0 _numberofdrops)
    (bind _id (CallFunction|RandomItemDropwithChance))
    (Utilities|Array|AddUnique (Variables|Default|GetItems_ID) _id)
    (bind _returnvalue_6 (Utilities|GetDataTableRow "/Game/Blueprints/Data/HumanParts/HumanParts_DataTable.HumanParts_DataTable" (Utilities|String|StringToName (Utilities|String|ToString(Integer) _id)))
      (:then
        (Game|SpawnActorfromClass (.class _returnvalue_6) (Math|Transform|MakeTransform (+ (Transformation|GetActorLocation) _returnvalue_5)) "AdjustIfPossibleButAlwaysSpawn" 0 (.itemid _returnvalue_6) (.thumbnail _returnvalue_6) (.name _returnvalue_6) (.maxstackssize _returnvalue_6) 0))))
  (if (== _plasmadrop 0)
    (Actor|DestroyActor)
    (else
      (for _index_2 (range 1 _plasmadrop)
        (Components|InstancedStaticMesh|AddInstance (Variables|Default|GetPlasma) (Math|Transform|MakeTransform _returnvalue_5 "0, 0, 0" "0.250000,0.250000,0.250000"))))))

(fn ConstructionScript)

(fn RandomMaxDropwithChance
  (params (Array :type Array%20of%20Integers))
  (Variables|Default|SetRandom (Math|Random|RandomIntegerinRange 0 100))
  (Variables|Default|SetProbSubtraction 100)
  (bind (_array_element _array_index) (Utilities|Array|ForEachLoopwithBreak Array :!label _label)
    (:LoopBody
      (bind _output_get (Variables|Default|SetProbSubtraction (- (Variables|Default|GetProbSubtraction) _array_element)))
      (if (>= (Variables|Default|GetRandom) _output_get)
        (Variables|Default|SetNumberOfDrops (- (Utilities|Array|Length Array) _array_index))
        (goto _label Break)
        (else
          (Variables|Default|SetNumberOfDrops 0))))
    (:Completed
      (return (Variables|Default|GetNumberOfDrops)))))

(fn RandomItemDropwithChance
  (Variables|Default|SetRandom (Math|Random|RandomIntegerinRange 0 100))
  (Variables|Default|SetProbSubtraction 100)
  (bind (_array_element _array_index) (Utilities|Array|ForEachLoopwithBreak (Variables|Default|GetItemsIDChance) :!label _label)
    (:LoopBody
      (bind _output_get (Variables|Default|SetProbSubtraction (- (Variables|Default|GetProbSubtraction) _array_element)))
      (if (>= (Variables|Default|GetRandom) _output_get)
        (Variables|Default|SetItemId_Drop (Utilities|Array|Get(acopy) (Variables|Default|GetItemsID_Drops) _array_index))
        (goto _label Break)
        (else
          (Variables|Default|SetItemId_Drop 0))))
    (:Completed
      (return (Variables|Default|GetItemId_Drop)))))