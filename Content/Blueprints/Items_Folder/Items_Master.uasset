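; Base pickup item actor that shows its texture on a thumbnail sprite and adds itself to the player's inventory on touch.
; When the player overlaps the sphere, ItemID selects the 100-series or 200-series stack array, with the ID minus that base as the index.
; Below the player's max hold, the stack increments and the item destroys itself; otherwise it prints a max-stack message and remains.
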(event OnComponentBeginOverlap(Sphere)
  (params (OverlappedComponent :type Primitive%20Component%20Object%20Reference) (OtherActor :type Actor%20Object%20Reference) (OtherComp :type Primitive%20Component%20Object%20Reference) (OtherBodyIndex :type Integer) (bFromSweep :type Boolean) (SweepResult :type Hit%20Result%20Structure%20%28by%20ref%29))
  (bind _itemid (Variables|Default|GetItemID))
  (bind _returnvalue (- _itemid 100))
  (bind _returnvalue_2 (- _itemid 200))
  (bind _asmain_player_blueprint (Utilities|Casting|CastToMainPlayer_Blueprint OtherActor))
  (if (>= _itemid 200)
    (if (>= (Utilities|Array|Get(acopy) (.items200stacks (Variables|/Game/Blueprints/Character/MainPlayer_Blueprint.MainPlayer_Blueprint_C|GetPlayerInventory _asmain_player_blueprint)) _returnvalue_2) (Variables|/Game/Blueprints/Character/MainPlayer_Blueprint.MainPlayer_Blueprint_C|GetMaxItemsHold _asmain_player_blueprint))
      (Development|PrintString (Utilities|String|Append (Utilities|String|ToString(Name) (Variables|Default|GetItemName)) "Has max stacks") :!label _label)
      (else
        (Utilities|Array|SetArrayElem (.items200stacks (Variables|/Game/Blueprints/Character/MainPlayer_Blueprint.MainPlayer_Blueprint_C|GetPlayerInventory _asmain_player_blueprint)) _returnvalue_2 (+ (Utilities|Array|Get(acopy) (.items200stacks (Variables|/Game/Blueprints/Character/MainPlayer_Blueprint.MainPlayer_Blueprint_C|GetPlayerInventory _asmain_player_blueprint)) _returnvalue_2) 1))
        (Actor|DestroyActor :!label _label_2)))
    (elif (>= (Utilities|Array|Get(acopy) (.items100stacks (Variables|/Game/Blueprints/Character/MainPlayer_Blueprint.MainPlayer_Blueprint_C|GetPlayerInventory _asmain_player_blueprint)) _returnvalue) (Variables|/Game/Blueprints/Character/MainPlayer_Blueprint.MainPlayer_Blueprint_C|GetMaxItemsHold _asmain_player_blueprint))
      (goto _label)
      (else
        (Utilities|Array|SetArrayElem (.items100stacks (Variables|/Game/Blueprints/Character/MainPlayer_Blueprint.MainPlayer_Blueprint_C|GetPlayerInventory _asmain_player_blueprint)) _returnvalue (+ (Utilities|Array|Get(acopy) (.items100stacks (Variables|/Game/Blueprints/Character/MainPlayer_Blueprint.MainPlayer_Blueprint_C|GetPlayerInventory _asmain_player_blueprint)) _returnvalue) 1))
        (goto _label_2)))))

(event EventBeginPlay
  (Rendering|Components|Sprite|SetSprite (Variables|Default|GetThumbnail) (Variables|Default|GetItemTexture)))

(event Collision|EventActorBeginOverlap
  (params (OtherActor :type Actor%20Object%20Reference)))

(event EventTick
  (params (DeltaSeconds :type Float%20%28single-precision%29)))

(fn ConstructionScript)