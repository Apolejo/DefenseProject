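; Fog of war actor whose mesh shows fog that can be revealed at given 2D locations.
; On BeginPlay it creates a render target cleared to black, dynamic instances of the subtract and fog materials, and makes the mesh visible.
; DrawSubtract passes a location to the subtract material, draws it into the render target, and feeds that texture to the fog material as its mask.
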(event Custom|DrawSubtract
  (params (LocationToDraw :type Vector%202D%20Structure))
  (bind _rendertarget (Variables|Default|GetRenderTarget))
  (Rendering|Material|SetVectorParameterValue (Variables|Default|GetSubtractMi) "DrawLocation" (Math|Conversions|ToLinearColor(Vector) (Math|Conversions|ToVector(Vector2D) LocationToDraw)) :!class /Script/Engine.MaterialInstanceDynamic)
  (Rendering|DrawMaterialtoRenderTarget _rendertarget (Variables|Default|GetSubtractMi))
  (Rendering|Material|SetTextureParameterValue (Variables|Default|GetFogOfWarMaterial) "RenderTargetTexture" _rendertarget))

(event EventBeginPlay
  (bind _returnvalue (Rendering|Material|CreateDynamicMaterialInstance "/Game/Materials/SubtractFog_Mat.SubtractFog_Mat" "None" :!class /Script/Engine.KismetMaterialLibrary))
  (Variables|Default|SetSubtractMi _returnvalue)
  (bind _returnvalue_2 (Rendering|CreateRenderTarget2D 1024 1024 "RTF_RGBA16f"))
  (Variables|Default|SetRenderTarget _returnvalue_2)
  (bind _returnvalue_3 (Rendering|Material|CreateDynamicMaterialInstance (Variables|Default|GetStaticMesh) 0 "/Game/Materials/Fog_Mat.Fog_Mat" "None" :!class /Script/Engine.PrimitiveComponent))
  (Variables|Default|SetFogOfWarMaterial _returnvalue_3)
  (Rendering|ClearRenderTarget2D (Variables|Default|GetRenderTarget))
  (Rendering|SetVisibility (Variables|Default|GetStaticMesh) true false))

(fn ConstructionScript)