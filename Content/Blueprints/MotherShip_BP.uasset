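; Player mothership base with health, a timeline-recharged shield, a building zone and an invisibility field; losing all life ends the game.
; Clicking it when nearby opens its upgrade UI, and UpdateMotherShip checks item costs for tiered field, shield, life and recharge upgrades.
; Field upgrades animate the radius across the range, building zone and a material parameter collection, while overlapping buildings get their invisibility setup.
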(event OnComponentBeginOverlap(InvisibilityRange)
  (params (OverlappedComponent :type Primitive%20Component%20Object%20Reference) (OtherActor :type Actor%20Object%20Reference) (OtherComp :type Primitive%20Component%20Object%20Reference) (OtherBodyIndex :type Integer) (bFromSweep :type Boolean) (SweepResult :type Hit%20Result%20Structure%20%28by%20ref%29))
  (Default|CallBuildingInvisible))

(event OnBeginCursorOver(MotherShip)
  (params (TouchedComponent :type Primitive%20Component%20Object%20Reference))
  (if (not (Variables|Default|GetIsPlayerCloser?))
    (Rendering|SetRenderCustomDepth TouchedComponent true)))

(event OnEndCursorOver(MotherShip)
  (params (TouchedComponent :type Primitive%20Component%20Object%20Reference))
  (if (not (Variables|Default|GetIsPlayerCloser?))
    (Rendering|SetRenderCustomDepth TouchedComponent false)))

(event OnComponentBeginOverlap(PlayerDetection)
  (params (OverlappedComponent :type Primitive%20Component%20Object%20Reference) (OtherActor :type Actor%20Object%20Reference) (OtherComp :type Primitive%20Component%20Object%20Reference) (OtherBodyIndex :type Integer) (bFromSweep :type Boolean) (SweepResult :type Hit%20Result%20Structure%20%28by%20ref%29))
  (bind _asmain_player_blueprint (Utilities|Casting|CastToMainPlayer_Blueprint OtherActor))
  (Variables|Default|SetIsPlayerCloser? true)
  (Rendering|SetRenderCustomDepth (Variables|Default|GetMotherShip) true)
  (Default|UpdateMotherShipInventory _asmain_player_blueprint))

(event OnComponentEndOverlap(PlayerDetection)
  (params (OverlappedComponent :type Primitive%20Component%20Object%20Reference) (OtherActor :type Actor%20Object%20Reference) (OtherComp :type Primitive%20Component%20Object%20Reference) (OtherBodyIndex :type Integer))
  (Utilities|Casting|CastToMainPlayer_Blueprint OtherActor)
  (Variables|Default|SetIsPlayerCloser? false)
  (Rendering|SetRenderCustomDepth (Variables|Default|GetMotherShip) false)
  (Widget|SetVisibility (Variables|References|GetMothershipUI_REF) "Hidden"))

(event OnClicked(MotherShip)
  (params (TouchedComponent :type Primitive%20Component%20Object%20Reference) (ButtonPressed :type Key%20Structure))
  (if (Variables|Default|GetIsPlayerCloser?)
    (Widget|SetVisibility (Variables|References|GetMothershipUI_REF) "Visible")
    (else
      (Development|PrintString "Need to get closer"))))

(event Custom|UpdateInvisibility
  ;[1 1 1] BeginPlay
  (for _array_element (Collision|GetOverlappingActors (Variables|Components|GetInvisibilityRange) "/Game/Blueprints/Buldings/BuildingMaster_BP.BuildingMaster_BP_C" :!class /Script/Engine.PrimitiveComponent)
    (bind _asbuilding_master_bp (Utilities|Casting|CastToBuildingMaster_BP _array_element))
    (Default|SetupInvisibility _asbuilding_master_bp)))

(event Custom|UpdateLife
  (params (LifePoints :type Float%20%28single-precision%29))
  ;[1 1 1] UpdateLife
  (if (> (Variables|Default|GetLifePoints) 0.0)
    (if (> (Variables|Default|GetShieldPoints) 0.0)
      (Variables|Default|SetShieldPoints (- (Variables|Default|GetShieldPoints) LifePoints))
      (if (> (Variables|Default|GetShieldPoints) 0.0)
        (CallFunction|RechargeShield :!label _label)
        (else
          (Variables|Default|SetLifePoints (- (Variables|Default|GetLifePoints) (Variables|Default|GetShieldPoints)))
          (Variables|Default|SetShieldPoints 0.0)
          (if (> (Variables|Default|GetLifePoints) 0.0) :!label _label_2
            (goto _label)
            (else
              (Default|ENDGAME (Variables|References|GetPlayerController_REF))))))
      (else
        (Variables|Default|SetLifePoints (- (Variables|Default|GetLifePoints) LifePoints))
        (goto _label_2)))
    (else
      (Default|ENDGAME (Variables|References|GetPlayerController_REF)))))

(event Custom|RechargeShield
  ;[1 1 1] RechargeShield
  (Variables|Default|SetShieldPointControl (Variables|Default|GetShieldPoints))
  (Utilities|FlowControl|RetriggerableDelay (Variables|Update|GetRechargeDelay))
  (Components|Timeline|SetPlayRate (Variables|Default|GetRecharge) (/ 1.0 (Variables|Update|GetRechargeTime)))
  (bind _rechargerate (Timeline|Recharge PlayFromStart)
    (:Update
      (Variables|Default|SetShieldPoints (Math|Float|Lerp (Variables|Default|GetShieldPointControl) (Variables|Update|GetShieldPointsCap) _rechargerate)))))

(event Custom|UpgradeShield
  (bind _invisibilityrange (Variables|Components|GetInvisibilityRange))
  (bind _returnvalue (Transformation|GetWorldTransform _invisibilityrange))
  (Variables|Default|SetScaleVector (.scale _returnvalue))
  (Variables|Default|SetRadius (Variables|Default|GetFinalRadius))
  (Variables|Default|SetShieldTimelineControl false)
  (bind _updatetheshield (Timeline|Shield PlayFromStart)
    (:Update
      (Transformation|SetWorldTransform (Variables|Components|GetInvisibilityRange) (Math|Transform|MakeTransform (.location _returnvalue) (.rotation _returnvalue) (Math|Vector|Lerp(Vector) (Variables|Default|GetScaleVector) (* (Variables|Default|GetScaleVector) (Variables|Update|GetInvisibilityUpgradeSize)) _updatetheshield)) false false)
      (Rendering|Material|SetScalarParameterValue "/Game/Materials/Effects/ParameterCollection/Cut_Collection_PM.Cut_Collection_PM" "Radius" (Math|Float|Lerp (Variables|Default|GetRadius) (* (Variables|Default|GetRadius) (Variables|Update|GetInvisibilityUpgradeSize)) _updatetheshield) :!class /Script/Engine.KismetMaterialLibrary)
      (Components|Sphere|SetSphereRadius (Variables|Components|GetInvisibilityField) (Math|Float|Lerp (Variables|Default|GetRadius) (* (Variables|Default|GetRadius) (Variables|Update|GetInvisibilityUpgradeSize)) _updatetheshield) false)
      (Default|UpdateBuildingRadius (Variables|Components|GetBuildingZone_Component) (Math|Float|Lerp (Variables|Default|GetRadius) (* (Variables|Default|GetRadius) (Variables|Update|GetInvisibilityUpgradeSize)) _updatetheshield))
      (Variables|Default|SetFinalRadius (Math|Float|Lerp (Variables|Default|GetRadius) (* (Variables|Default|GetRadius) (Variables|Update|GetInvisibilityUpgradeSize)) _updatetheshield)))
    (:Finished
      (Variables|Default|SetShieldTimelineControl true))))

(event EventBeginPlay
  ;[1 1 1] BeginPlay
  (CallFunction|SetupUIReference)
  (EventDispatchers|BindEventtoBuildingInvisible (delegate Custom|UpdateInvisibility))
  (Default|UpdateBuildingRadius (Variables|Components|GetBuildingZone_Component) (Variables|Default|GetRadius))
  (Variables|Default|SetLifePoints (Variables|Update|GetLifePointsCap))
  (Variables|Default|SetShieldPoints (Variables|Update|GetShieldPointsCap))
  (bind _asplayer_game_controller (Utilities|Casting|CastToPlayerGameController (Game|GetPlayerController 0)))
  (Variables|References|SetPlayerController_REF _asplayer_game_controller)
  (Utilities|FlowControl|Delay 0.2)
  (Variables|References|SetMainHudREF (Variables|/Game/Blueprints/PlayerGameController.PlayerGameController_C|GetMainHud_Ref _asplayer_game_controller))
  (Variables|References|SetMothershipUI_REF (Variables|/Game/Blueprints/UserInterface/MainUI_Widget.MainUI_Widget_C|GetMothership_UI_WBP (Variables|/Game/Blueprints/PlayerGameController.PlayerGameController_C|GetMainHud_Ref _asplayer_game_controller)))
  (Variables|/Game/Blueprints/UserInterface/Mothership_UI_WBP.Mothership_UI_WBP_C|SetMothership_REF (Variables|/Game/Blueprints/UserInterface/MainUI_Widget.MainUI_Widget_C|GetMothership_UI_WBP (Variables|/Game/Blueprints/PlayerGameController.PlayerGameController_C|GetMainHud_Ref _asplayer_game_controller)) self)
  (Variables|/Game/Blueprints/UserInterface/Mothership_UI_WBP.Mothership_UI_WBP_C|SetMotherShipName (Variables|/Game/Blueprints/UserInterface/MainUI_Widget.MainUI_Widget_C|GetMothership_UI_WBP (Variables|/Game/Blueprints/PlayerGameController.PlayerGameController_C|GetMainHud_Ref _asplayer_game_controller)) "ChinaNumberOne")
  (Rendering|Material|SetVectorParameterValue "/Game/Materials/Effects/ParameterCollection/Cut_Collection_PM.Cut_Collection_PM" "Position" (Math|Conversions|ToLinearColor(Vector) (Transformation|GetWorldLocation (Variables|Components|GetInvisibilityRange))) :!class /Script/Engine.KismetMaterialLibrary)
  (Rendering|Material|SetScalarParameterValue "/Game/Materials/Effects/ParameterCollection/Cut_Collection_PM.Cut_Collection_PM" "Radius" (Variables|Default|GetRadius) :!class /Script/Engine.KismetMaterialLibrary))

(event Collision|EventActorBeginOverlap
  (params (OtherActor :type Actor%20Object%20Reference)))

(event EventTick
  (params (DeltaSeconds :type Float%20%28single-precision%29)))

(fn ConstructionScript)

(fn UpdateMotherShip
  (params (UpgradeID :type Integer) (Tier :type Integer) (ItemsNeeded :type Integer) (ItemID :type Integer) (CanBeUpgraded? :type Boolean))
  (if (< (Utilities|Array|Get(acopy) (Variables|/Game/Blueprints/PlayerGameController.PlayerGameController_C|Get200Stacks (Variables|References|GetPlayerController_REF)) ItemID) ItemsNeeded)
    (Development|PrintString "Insufficent Items")
    (return false)
    (else
      (switch int UpgradeID
        (:0
          (|InvisibilityUpgrade Tier
            (:then
              _)
            (:then2
              _)
            (:then3
              _)))
        (:1
          (|ShieldUpgrade Tier
            (:then
              _)
            (:then2
              _)
            (:then3
              _))
          (CallFunction|RechargeShield))
        (:2
          (|LifeUpgrade Tier
            (:then
              _)
            (:then2
              _)
            (:then3
              _)))
        (:3
          (|RechargeDelayUpgrade Tier
            (:then
              _)
            (:then2
              _)
            (:then3
              _)))
        (:4
          (|RechargeTimeUpgrade Tier
            (:then
              _)
            (:then2
              _)
            (:then3
              _))))
      (Default|UpdateInventoryStacks (Variables|References|GetPlayerController_REF) (+ ItemID 200) (* ItemsNeeded -1))
      (return true))))

(fn SetupUIReference
  (bind _ashp_shield_bar_wbp (Utilities|Casting|CastToHpShieldBar_WBP (UserInterface|GetUserWidgetObject (Variables|Default|GetHP/Shield))))
  (Variables|/Game/Blueprints/UserInterface/BuildingsWidget/HpShieldBar_WBP.HpShieldBar_WBP_C|SetActor _ashp_shield_bar_wbp self))

(fn GetCurrentHP
  (return (Variables|Default|GetLifePoints) (Variables|Update|GetLifePointsCap) (Variables|Default|GetShieldPoints) (Variables|Update|GetShieldPointsCap)))

(fn GetCurrentPower
  (return 0.0))

(fn GetMaxPower
  (return 0.0))