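; Base building actor with hover outlines, proximity-gated selection through the HUD and recycling that returns resources through the controller.
; Child hooks activate or deactivate work as connection and energy state change, toggling an out-of-energy widget.
; Completed buildings pass cable-spot clicks to the controller for wiring.
; Upgrade checks move inventory items into the upgrade widget's requirements, then swap the building for an upgrade ghost once all are met.
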(event OnBeginCursorOver(StaticMesh)
  (params (TouchedComponent :type Primitive%20Component%20Object%20Reference))
  ;[1 1 1] MouseOverlay
  (if (not (Variables|NottoTouch|GetClicked?))
    (Rendering|SetRenderCustomDepth TouchedComponent true)))

(event OnEndCursorOver(StaticMesh)
  (params (TouchedComponent :type Primitive%20Component%20Object%20Reference))
  ;[1 1 1] MouseOverlay
  (if (not (Variables|NottoTouch|GetClicked?))
    (Rendering|SetRenderCustomDepth TouchedComponent false)))

(event OnComponentBeginOverlap(Hitbox)
  (params (OverlappedComponent :type Primitive%20Component%20Object%20Reference) (OtherActor :type Actor%20Object%20Reference) (OtherComp :type Primitive%20Component%20Object%20Reference) (OtherBodyIndex :type Integer) (bFromSweep :type Boolean) (SweepResult :type Hit%20Result%20Structure%20%28by%20ref%29))
  ;[1 1 1] PlayerCloser
  (if (Variables|NottoTouch|GetIsBuildingCompleted?)
    (if (.bSuccess (Utilities|Casting|CastToMainPlayer_Blueprint OtherActor))
      (Variables|NottoTouch|SetImCloser? true)
      (Rendering|SetRenderCustomDepth (Variables|Default|GetStaticMesh) true)
      (Rendering|SetVisibility (Variables|Default|GetUpgradeWidget) true false))))

(event OnComponentEndOverlap(Hitbox)
  (params (OverlappedComponent :type Primitive%20Component%20Object%20Reference) (OtherActor :type Actor%20Object%20Reference) (OtherComp :type Primitive%20Component%20Object%20Reference) (OtherBodyIndex :type Integer))
  ;[1 1 1] PlayerCloser
  (if (Variables|NottoTouch|GetIsBuildingCompleted?)
    (if (.bSuccess (Utilities|Casting|CastToMainPlayer_Blueprint OtherActor))
      (Variables|NottoTouch|SetImCloser? false)
      (Rendering|SetRenderCustomDepth (Variables|Default|GetStaticMesh) false)
      (Rendering|SetVisibility (Variables|Default|GetUpgradeWidget) false false)
      (if (Variables|NottoTouch|GetClicked?)
        (CallFunction|SetClickedOff)))))

(event OnClicked(Cable_SpotA)
  (params (TouchedComponent :type Primitive%20Component%20Object%20Reference) (ButtonPressed :type Key%20Structure))
  (if (Variables|NottoTouch|GetIsBuildingCompleted?)
    (Default|CableInformation (Variables|References|GetControllerRef) (Transformation|GetWorldLocation TouchedComponent) self)))

(event OnClicked(Cable_SpotB)
  (params (TouchedComponent :type Primitive%20Component%20Object%20Reference) (ButtonPressed :type Key%20Structure))
  (if (Variables|NottoTouch|GetIsBuildingCompleted?)
    (Default|CableInformation (Variables|References|GetControllerRef) (Transformation|GetWorldLocation TouchedComponent) self)))

(event Custom|CreateWidgetByClick
  ;[1 1 1] SetupWidgetOnClick
  (if (Variables|NottoTouch|GetImCloser?)
    (if (not (Variables|NottoTouch|GetClicked?))
      (Variables|NottoTouch|SetClicked? true)
      (CallFunction|DetectifWidgetUpandCreateOne))
    (else
      (Development|PrintString "get closer"))))

(event Custom|RecycleBuilding
  ;[1 1 1] ReturnResourcesWhenRecycled
  (CallFunction|DestroyandReturnResources (Variables|References|GetMainHudREF)))

(event Custom|SetClickedOff
  (bind _mainhudref (Variables|References|GetMainHudREF))
  (Widget|SetVisibility (Variables|/Game/Blueprints/UserInterface/MainUI_Widget.MainUI_Widget_C|GetSelectBuilding_UI _mainhudref) "Hidden")
  (Default|SelectBuildingWidgetSetup _mainhudref)
  (Rendering|SetRenderCustomDepth (Variables|Default|GetStaticMesh) false)
  (Variables|NottoTouch|SetClicked? false))

(event Custom|BuildingOutOfEnergy
  ;[1 1 1] ActiveFunctions
  (Rendering|SetVisibility (Variables|Default|GetOutOfEnergy_Widget) true false)
  (if (Variables|NottoTouch|GetImActive?)
    (CallFunction|DeactivateWorkingBuilding)
    (Variables|NottoTouch|SetImActive? false)))

(event Custom|BuildingActive
  (bind _outofenergy_widget (Variables|Default|GetOutOfEnergy_Widget))
  ;[1 1 1] ActiveFunctions
  (if (Variables|NottoTouch|GetImConected?)
    (Rendering|SetVisibility _outofenergy_widget false false)
    (if (not (Variables|NottoTouch|GetImActive?))
      (CallFunction|ActivateWorkingBuilding)
      (Variables|NottoTouch|SetImActive? true))
    (else
      (Rendering|SetVisibility _outofenergy_widget true false)
      (if (Variables|NottoTouch|GetImActive?)
        (CallFunction|DeactivateWorkingBuilding)
        (Variables|NottoTouch|SetImActive? false)))))

(event Custom|CheckUpgrade
  (params (ItemID :type Integer))
  (bind _upgradewidget_ref (Variables|References|GetUpgradeWidget_Ref))
  ;[1 1 1] Upgrade
  (if (Variables|NottoTouch|GetIsBuildingCompleted?)
    (Utilities|IsValid _upgradewidget_ref
      (:Is%20Valid
        (bind (_array_element _array_index) (Utilities|Array|ForEachLoopwithBreak (Variables|/Game/Blueprints/UserInterface/UpgradeWidget/UpgradeItemList_Widget.UpgradeItemList_Widget_C|GetItemNeededArray _upgradewidget_ref) :!label _label)
          (:LoopBody
            (Utilities|Array|SetArrayElem (Variables|Upgrade|GetUpgradeParts) _array_index (== _array_element 0))
            (if (not (== _array_element 0))
              (if (<= (Utilities|Array|Get(acopy) (Variables|/Game/Blueprints/PlayerGameController.PlayerGameController_C|Get200Stacks (Variables|References|GetControllerRef)) _array_index) 0)
                (Development|PrintString "InsufficientMaterials")
                (else
                  ;;[1 1 1] ReduceItemStacks
                  (Default|DecreaseItemsNeeded _upgradewidget_ref _array_index 1)
                  (Default|UpdateInventoryStacks (Variables|References|GetControllerRef) (+ _array_index 200) -1)
                  (goto _label Break)))))
          (:Completed
            (if (not (Utilities|Array|ContainsItem (Variables|Upgrade|GetUpgradeParts) false))
              (Utilities|FlowControl|DoOnce false
                (:Completed
                  (CallFunction|DoUpgradewhenEverthingIsTrue))))))))))

(event Custom|DoUpgradeWhenEverthingIsTrue
  ;[1 1 1] Upgrade
  ;;[1 0 0] UpgradeMechanic
  (Game|SpawnActorfromClass "/Game/Blueprints/Buldings/BuildingUpgradeGhost_BP.BuildingUpgradeGhost_BP_C" (Transformation|GetActorTransform) "Undefined" 0 (Variables|UpgradeSettings|GetBuildingClass_Upgrade) (Variables|References|GetControllerRef) (Variables|UpgradeSettings|GetUpgradeDelayTimer) (Variables|UpgradeSettings|GetMeshUpgradeGhost) 0)
  (Actor|DestroyActor))

(event Custom|DeactivateWorkingBuilding)

(event Custom|ActivateWorkingBuilding)

(event EventBeginPlay
  ;[1 1 1] BeginPlaySetup
  (bind _asplayer_game_controller (Utilities|Casting|CastToPlayerGameController (Game|GetPlayerController 0)))
  (Variables|References|SetControllerRef _asplayer_game_controller)
  (Variables|References|SetMainHudREF (Variables|/Game/Blueprints/PlayerGameController.PlayerGameController_C|GetMainHud_Ref _asplayer_game_controller))
  (bind _asupgrade_item_list_widget (Utilities|Casting|CastToUpgradeItemList_Widget (UserInterface|GetUserWidgetObject (Variables|Default|GetUpgradeWidget))))
  (bind _output_get (Variables|References|SetUpgradeWidget_Ref _asupgrade_item_list_widget))
  (Variables|/Game/Blueprints/UserInterface/UpgradeWidget/UpgradeItemList_Widget.UpgradeItemList_Widget_C|SetItemNeededArray _output_get (Utilities|Array|MakeArray (Variables|UpgradeItems|GetUpgradeItem1) (Variables|UpgradeItems|GetUpgradeItem2) (Variables|UpgradeItems|GetUpgradeItem3) (Variables|UpgradeItems|GetUpgradeItem4) (Variables|UpgradeItems|GetUpgradeItem5) (Variables|UpgradeItems|GetUpgradeItem6)))
  (Variables|Cost|SetEnergyConsumption (* (Variables|Cost|GetEnergyConsumption) (Variables|UpgradeSettings|GetEnergyUsageMultiplier))))

(fn ConstructionScript
  (Components|StaticMesh|SetStaticMesh (Variables|Default|GetStaticMesh) (Variables|Components|GetDisplayMesh)))

(fn DetectifWidgetUpandCreateOne
  (bind _mainhudref (Variables|References|GetMainHudREF))
  (bind _selectbuilding_ui (Variables|/Game/Blueprints/UserInterface/MainUI_Widget.MainUI_Widget_C|GetSelectBuilding_UI _mainhudref))
  (if (Widget|IsVisible _selectbuilding_ui)
    (Default|SelectBuildingWidgetSetup _mainhudref)
    (Default|TurnOffOverlay _selectbuilding_ui)
    (return)
    (else
      (Variables|/Game/Blueprints/UserInterface/SelectBuilding_UI.SelectBuilding_UI_C|SetBuildingRef _selectbuilding_ui self)
      (Widget|SetVisibility _selectbuilding_ui "Visible")
      (Variables|/Game/Blueprints/UserInterface/SelectBuilding_UI.SelectBuilding_UI_C|SetBuildingName _selectbuilding_ui (Variables|Default|GetBuildingName))
      (Rendering|SetRenderCustomDepth (Variables|Default|GetStaticMesh) true)
      (Default|SelectBuildingWidgetSetup _mainhudref)
      (return))))

(fn DestroyandReturnResources
  (params (MainHud :type Main%20UI%20Widget%20Object%20Reference))
  (Rendering|SetRenderCustomDepth (Variables|Default|GetStaticMesh) false)
  (Widget|SetVisibility (Variables|/Game/Blueprints/UserInterface/MainUI_Widget.MainUI_Widget_C|GetSelectBuilding_UI MainHud) "Hidden")
  (Default|ReturnResource (Variables|References|GetControllerRef) 0.5 self)
  (Actor|DestroyActor))