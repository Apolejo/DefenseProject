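; Placement preview actor for build mode that shows the selected building's mesh at the grid-snapped cursor position.
; ConstructBuildings briefly spawns the building class to copy its mesh, costs, tags, hitbox and timing, then destroys it.
; While active, a gated Tick moves the ghost and swaps valid/error materials, requiring a matching build zone tag and no overlapping buildings, proxies or characters.
; GetConstructionStruct packages the placement data for construction.
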(event OnComponentBeginOverlap(GhostBuildStaticMesh)
  (params (OverlappedComponent :type Primitive%20Component%20Object%20Reference) (OtherActor :type Actor%20Object%20Reference) (OtherComp :type Primitive%20Component%20Object%20Reference) (OtherBodyIndex :type Integer) (bFromSweep :type Boolean) (SweepResult :type Hit%20Result%20Structure%20%28by%20ref%29))
  (bind (_asfarming_zone_bp _bsuccess) (Utilities|Casting|CastToFarmingZone_BP OtherActor))
  (bind (_asdefensive_zone_bp _bsuccess_2) (Utilities|Casting|CastToDefensiveZone_BP OtherActor))
  (bind (_asoffensive_zone_bp _bsuccess_3) (Utilities|Casting|CastToOffensiveZone_BP OtherActor))
  (bind (_asdecorative_zone_bp _bsuccess_4) (Utilities|Casting|CastToDecorativeZone_BP OtherActor))
  ;[1 0 0] Check overlap (BETTER TRY TO GET A MOST OPTIMIZED WAY)
  (if _bsuccess
    (Variables|Zone|SetResourceZone (Variables|/Game/Blueprints/Buldings/BuildingZones/BuildingZone_Master.BuildingZone_Master_C|GetResource_Zone _asfarming_zone_bp))
    (elif _bsuccess_2
      (Variables|Zone|SetDefensiveZone (Variables|/Game/Blueprints/Buldings/BuildingZones/BuildingZone_Master.BuildingZone_Master_C|GetDefensive_Zone _asdefensive_zone_bp))
      (elif _bsuccess_3
        (Variables|Zone|SetOffensiveZone (Variables|/Game/Blueprints/Buldings/BuildingZones/BuildingZone_Master.BuildingZone_Master_C|GetOffensive_Zone _asoffensive_zone_bp))
        (elif _bsuccess_4
          (Variables|Zone|SetDecorativeZone (Variables|/Game/Blueprints/Buldings/BuildingZones/BuildingZone_Master.BuildingZone_Master_C|GetDecorative_Zone _asdecorative_zone_bp)))))))

(event OnComponentEndOverlap(GhostBuildStaticMesh)
  (params (OverlappedComponent :type Primitive%20Component%20Object%20Reference) (OtherActor :type Actor%20Object%20Reference) (OtherComp :type Primitive%20Component%20Object%20Reference) (OtherBodyIndex :type Integer))
  ;[1 0 0] Check overlap (BETTER TRY TO GET A MOST OPTIMIZED WAY)
  (if (.bSuccess (Utilities|Casting|CastToFarmingZone_BP OtherActor))
    (Variables|Zone|SetResourceZone false)
    (elif (.bSuccess (Utilities|Casting|CastToDefensiveZone_BP OtherActor))
      (Variables|Zone|SetDefensiveZone false)
      (elif (.bSuccess (Utilities|Casting|CastToOffensiveZone_BP OtherActor))
        (Variables|Zone|SetOffensiveZone false)
        (elif (.bSuccess (Utilities|Casting|CastToDecorativeZone_BP OtherActor))
          (Variables|Zone|SetDecorativeZone false))))))

(event Custom|OnSpawn
  (params (DisplayMesh :type Static%20Mesh%20Object%20Reference) (BuildingClass :type Building%20Master%20BP%20Class%20Reference) (ConstructionProxy :type Construction%20Proxy%20BP%20Class%20Reference) (Time :type Float%20%28single-precision%29) (BuildTags :type Array%20of%20Names) (WallOrFloor :type ETraceTypeQuery%20Enum :default "TraceTypeQuery1") (Hitbox :type Vector) (WoodCost :type Float%20%28single-precision%29) (MetalCost :type Float%20%28single-precision%29))
  ;[1 1 1] Spawn
  (if (not (Variables|Default|GetIsActive))
    (Variables|Default|SetBuildingClass BuildingClass)
    (Variables|Default|SetConstructionProxy ConstructionProxy)
    (Variables|ActorReference|SetDisplayMesh DisplayMesh)
    (Variables|ActorReference|SetTimeRequired Time)
    (Variables|Default|SetBuildingTags BuildTags)
    (Variables|ActorReference|SetPlaceableLocation WallOrFloor)
    (Variables|ActorReference|SetHitbox Hitbox)
    (Variables|ActorReference|SetWoodRequired WoodCost)
    (Variables|ActorReference|SetMetalRequired MetalCost)
    (Variables|Default|SetIsActive true)
    (Variables|/Game/Blueprints/PlayerGameController.PlayerGameController_C|SetBuildModeActive (Variables|Default|GetGameControllerRef) true)
    (Components|StaticMesh|SetStaticMesh (Variables|Default|GetGhostBuildStaticMesh) (Variables|ActorReference|GetDisplayMesh))
    (CallFunction|OpenTickGate)
    (CallFunction|SetMasterial (not (Variables|Default|GetIsOverlapping)))))

(event Custom|KillGhost
  ;[1 1 1] KillGhost
  (Variables|Default|SetBuildingClass 0)
  (Variables|Default|SetConstructionProxy 0)
  (Variables|ActorReference|SetTimeRequired 0.0)
  (Utilities|Array|Clear (Variables|Default|GetBuildingTags))
  (Variables|ActorReference|SetWoodRequired 0.0)
  (Variables|ActorReference|SetMetalRequired 0.0)
  (CallFunction|CloseTickGate)
  (Components|StaticMesh|SetStaticMesh (Variables|Default|GetGhostBuildStaticMesh) 0)
  (Variables|ActorReference|SetDisplayMesh 0)
  (Variables|Default|SetIsActive false)
  (Variables|/Game/Blueprints/PlayerGameController.PlayerGameController_C|SetBuildModeActive (Variables|Default|GetGameControllerRef) false))

(event Custom|OpenTickGate
  ;[1 1 1] Tick
  (Utilities|FlowControl|Gate true) ; enters at Open
)

(event Custom|CloseTickGate
  ;[1 1 1] Tick
  (Utilities|FlowControl|Gate true) ; enters at Close
)

(event Custom|SetMasterial
  (params (IsError :type Boolean))
  (bind _ghostbuildstaticmesh (Variables|Default|GetGhostBuildStaticMesh))
  ;[1 1 1] SetMaterialIfOverlap
  (if (not (Math|Boolean|Equal(Boolean) IsError (Variables|Default|GetIsOverlapping)))
    (bind _output_get (Variables|Default|SetIsOverlapping IsError))
    (if _output_get
      (Rendering|Material|SetMaterial _ghostbuildstaticmesh 0 "/Game/Materials/BuildingMaterials/M_Ghost_Material_ERROR.M_Ghost_Material_ERROR")
      (else
        (Rendering|Material|SetMaterial _ghostbuildstaticmesh 0 "/Game/Materials/BuildingMaterials/M_Ghost_Material_Place.M_Ghost_Material_Place")))))

(event EventConstructBuildings
  (params (MainBuilding :type Building%20Master%20BP%20Class%20Reference))
  ;[1 1 1] ConstructBuilding
  (bind _returnvalue (Game|SpawnActorfromClass MainBuilding (Math|Transform|MakeTransform (Variables|Default|GetCursorWorldPosition)) "Undefined" 0 (Variables|Default|GetGameControllerRef) 0))
  (Utilities|FlowControl|Sequence
    (:then_0
      (bind _asbuilding_master_bp (Utilities|Casting|CastToBuildingMaster_BPClass MainBuilding))
      (CallFunction|KillGhost)
      (CallFunction|OnSpawn (Variables|/Game/Blueprints/Buldings/BuildingMaster_BP.BuildingMaster_BP_C|GetDisplayMesh _returnvalue) _asbuilding_master_bp (Variables|/Game/Blueprints/Buldings/BuildingMaster_BP.BuildingMaster_BP_C|GetConstructionProxy _returnvalue) (Variables|/Game/Blueprints/Buldings/BuildingMaster_BP.BuildingMaster_BP_C|GetConstructionTime _returnvalue) (Variables|/Script/Engine.Actor|GetTags _returnvalue) (Variables|/Game/Blueprints/Buldings/BuildingMaster_BP.BuildingMaster_BP_C|GetTraceChannel _returnvalue) (Variables|/Script/Engine.BoxComponent|GetBoxExtent (Variables|/Game/Blueprints/Buldings/BuildingMaster_BP.BuildingMaster_BP_C|GetHitbox _returnvalue)) (Variables|/Game/Blueprints/Buldings/BuildingMaster_BP.BuildingMaster_BP_C|GetWoodCost _returnvalue) (Variables|/Game/Blueprints/Buldings/BuildingMaster_BP.BuildingMaster_BP_C|GetMetalCost _returnvalue)))
    (:then_1
      (Actor|DestroyActor _returnvalue))))

(event EventTick
  (params (DeltaSeconds :type Float%20%28single-precision%29))
  ;[1 1 1] Tick
  (Utilities|FlowControl|Gate true
    (:Exit
      (Transformation|SetActorLocation (CallFunction|SetGridSnapVector) false false)
      (if (CallFunction|CheckOverlap)
        (CallFunction|SetMasterial true)
        (else
          (CallFunction|SetMasterial false))))))

(fn ConstructionScript)

(fn SetCursorPosition
  (params (CursorLocation :type Vector))
  (Variables|Default|SetCursorWorldPosition CursorLocation)
  (return))

(fn SetGridSnapVector
  (bind _cursorworldposition (Variables|Default|GetCursorWorldPosition))
  (bind _gridsize (Variables|Default|GetGridSize))
  (return (Math|Vector|MakeVector (CallFunction|GridSnap (.x _cursorworldposition) _gridsize) (CallFunction|GridSnap (.y _cursorworldposition) _gridsize) (CallFunction|GridSnap (.z _cursorworldposition) _gridsize))))

(fn GetConstructionStruct
  (return (Utilities|Struct|MakeConstructionStruct (Variables|Default|GetBuildingClass) (Variables|Default|GetConstructionProxy) (Math|Transform|MakeTransform (Transformation|GetActorLocation) (Transformation|GetActorRotation)) (Variables|ActorReference|GetDisplayMesh) (Variables|ActorReference|GetHitbox) (Variables|ActorReference|GetTimeRequired))))

(fn CheckOverlap
  (bind _overlappingactors (Collision|GetOverlappingActors "/Game/Blueprints/Constructions/ConstructionProxy_BP.ConstructionProxy_BP_C" :!class /Script/Engine.Actor))
  (bind _overlappingactors_2 (Collision|GetOverlappingActors "/Game/Blueprints/Character/Character_Blueprint.Character_Blueprint_C" :!class /Script/Engine.Actor))
  (bind _overlappingactors_3 (Collision|GetOverlappingActors "/Game/Blueprints/Buldings/BuildingMaster_BP.BuildingMaster_BP_C" :!class /Script/Engine.Actor))
  (bind _buildingtags (Variables|Default|GetBuildingTags))
  (bind _returnvalue (Utilities|Array|Length _overlappingactors))
  (bind _returnvalue_2 (Utilities|Array|Length _overlappingactors_2))
  (bind _returnvalue_3 (Utilities|Array|Length _overlappingactors_3))
  (bind _returnvalue_4 (> _returnvalue_3 0))
  (bind _returnvalue_5 (> _returnvalue 0))
  (bind _returnvalue_6 (> _returnvalue_2 0))
  (if (Variables|Zone|GetDefensiveZone)
    (return (Math|Boolean|ORBoolean _returnvalue_4 _returnvalue_6 (not (Utilities|Array|ContainsItem _buildingtags "Defensive")) _returnvalue_5))
    (elif (Variables|Zone|GetOffensiveZone)
      (return (Math|Boolean|ORBoolean _returnvalue_4 _returnvalue_6 (not (Utilities|Array|ContainsItem _buildingtags "Offensive")) _returnvalue_5))
      (elif (Variables|Zone|GetResourceZone)
        (return (Math|Boolean|ORBoolean _returnvalue_4 _returnvalue_6 (not (Utilities|Array|ContainsItem _buildingtags "Resource")) _returnvalue_5))
        (elif (Variables|Zone|GetDecorativeZone)
          (return (Math|Boolean|ORBoolean _returnvalue_4 _returnvalue_6 (not (Utilities|Array|ContainsItem _buildingtags "Decorative")) _returnvalue_5))
          (else
            (return true)))))))