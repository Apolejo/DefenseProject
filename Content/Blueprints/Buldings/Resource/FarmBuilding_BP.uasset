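; Farm building that grows planted items from inventory into Food the player collects.
; PlantPlot, requiring a completed, active building, reads the Plots data table, consumes the item and sets timeline play rates from GrowTime.
; Plots grow once and clear on collection; trees mature over double time, then regrow fruit after each harvest.
; Timelines drive the progress display, stop on deactivation and resume on activation; ResourceCollected sends finished yields to the controller.
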(event Custom|PlantPlot
  (params (ItemID :type Integer))
  ;[1 1 1] GetPlotInformation
  (Variables|Default|SetItemID ItemID)
  (if (Variables|Default|GetIsBuildingCompleted?)
    (if (Variables|Default|GetImActive?)
      (if (Variables|Default|GetHasAlreadyAnItem?)
        (Development|PrintString "Has A Seed")
        (else
          (Variables|Default|SetHasAlreadyAnItem? true)
          (bind _returnvalue (Utilities|GetDataTableRow "/Game/Blueprints/Data/Plots_DataTable.Plots_DataTable" (Utilities|String|StringToName (Utilities|String|ToString(Integer) (Variables|Default|GetItemID))))
            (:then
              (Default|UpdateInventoryStacks (Variables|Default|GetControllerRef) (.itemid _returnvalue) -1)
              (bind _output_get (Variables|Default|SetIsAPlot? (.imaplot? _returnvalue)))
              (if _output_get
                (Variables|/Game/Blueprints/UserInterface/DynamicCircle_Widget.DynamicCircle_Widget_C|SetNameText (Variables|Default|GetLoading_Ref) (Utilities|Text|ToText(Name) (.foodname _returnvalue)))
                (Components|Timeline|SetPlayRate (Variables|Default|GetPlotGrowTime) (/ 1.0 (.growtime _returnvalue)))
                (Rendering|SetVisibility (Variables|Default|GetResourceLoad) true false)
                ;;[1 1 1] GrowUpMechanic
                (bind _plotgrow (Timeline|PlotGrowTime PlayFromStart) ; Plot
                  (:Update
                    (Default|SetProgress (Variables|Default|GetLoading_Ref) _plotgrow "(R=1.000000,G=1.000000,B=1.000000,A=1.000000)" "(R=0.000000,G=1.000000,B=0.109550,A=1.000000)"))
                  (:Finished
                    (Variables|Default|SetIsResourceComplete? true)
                    (Development|PrintString "GrowUp")
                    (Variables|Default|SetFood (* (Variables|Default|GetOutputMultiplier) (.foodvalue _returnvalue)))))
                (else
                  (Variables|/Game/Blueprints/UserInterface/DynamicCircle_Widget.DynamicCircle_Widget_C|SetNameText (Variables|Default|GetLoading_Ref) (Utilities|Text|ToText(Name) (.foodname _returnvalue)))
                  (Components|Timeline|SetPlayRate (Variables|Default|GetPlantGrowTime) (/ 1.0 (* (.growtime _returnvalue) 2.0)))
                  (Rendering|SetVisibility (Variables|Default|GetResourceLoad) true false)
                  (bind _plotgrow_2 (Timeline|PlantGrowTime PlayFromStart) ; Tree
                    (:Update
                      (Default|SetProgress (Variables|Default|GetLoading_Ref) _plotgrow_2 "(R=1.000000,G=1.000000,B=1.000000,A=1.000000)" "(R=0.274724,G=0.000000,B=1.000000,A=1.000000)"))
                    (:Finished
                      (Variables|Default|SetFullGrowUpTree true)
                      (Default|SetProgress (Variables|Default|GetLoading_Ref) 0.0)
                      (Components|Timeline|SetPlayRate (Variables|Default|GetFruitGrowTime) (/ 1.0 (.growtime _returnvalue)))
                      (bind _plotgrow_3 (Timeline|FruitGrowTime Play)
                        (:Update
                          (Default|SetProgress (Variables|Default|GetLoading_Ref) _plotgrow_3 "(R=1.000000,G=1.000000,B=1.000000,A=1.000000)" "(R=0.000000,G=1.000000,B=0.109550,A=1.000000)"))
                        (:Finished
                          (Variables|Default|SetIsResourceComplete? true)
                          (Development|PrintString "GrowUp")
                          (Variables|Default|SetFood (* (.foodvalue _returnvalue) (Variables|Default|GetOutputMultiplier)))))))))))))
      (else
        (Development|PrintString "NeedMoreEnergy")))))

(event Custom|ReGrowFruit
  ;[1 1 1] GetPlotInformation
  (Components|Timeline|SetPlayRate (Variables|Default|GetFruitGrowTime) (/ 1.0 (.growtime (stale Custom|PlantPlot _returnvalue))))
  (Rendering|SetVisibility (Variables|Default|GetResourceLoad) true false)
  (bind _plotgrow (Timeline|FruitGrowTime PlayFromStart)
    (:Update
      (Default|SetProgress (Variables|Default|GetLoading_Ref) _plotgrow "(R=1.000000,G=1.000000,B=1.000000,A=1.000000)" "(R=0.000000,G=1.000000,B=0.109550,A=1.000000)"))
    (:Finished
      (Variables|Default|SetIsResourceComplete? true)
      (Development|PrintString "GrowUp")
      (Variables|Default|SetFood (* (.foodvalue (stale Custom|PlantPlot _returnvalue)) (Variables|Default|GetOutputMultiplier))))))

(event EventBeginPlay
  (|CallParentFunction) ; This node is disabled and will not be called.\nDrag off pins to build functionality.
)

(event Collision|EventActorBeginOverlap
  (params (OtherActor :type Actor%20Object%20Reference))
  (|CallParentFunction OtherActor) ; This node is disabled and will not be called.\nDrag off pins to build functionality.
)

(event EventTick
  (params (DeltaSeconds :type Float%20%28single-precision%29))
  (|CallParentFunction DeltaSeconds) ; This node is disabled and will not be called.\nDrag off pins to build functionality.
)

(event EventDeactivateWorkingBuilding
  ;[1 1 1] GetPlotInformation
  (Utilities|FlowControl|Sequence
    (:then_0
      ;;[1 1 1] GrowUpMechanic
      (bind _plotgrow (Timeline|PlotGrowTime Stop) ; Plot
        (:Update
          (Default|SetProgress (Variables|Default|GetLoading_Ref) _plotgrow "(R=1.000000,G=1.000000,B=1.000000,A=1.000000)" "(R=0.000000,G=1.000000,B=0.109550,A=1.000000)"))
        (:Finished
          (Variables|Default|SetIsResourceComplete? true)
          (Development|PrintString "GrowUp")
          (Variables|Default|SetFood (* (Variables|Default|GetOutputMultiplier) (.foodvalue (stale Custom|PlantPlot _returnvalue)))))))
    (:then_1
      (bind _plotgrow_2 (Timeline|FruitGrowTime Stop)
        (:Update
          (Default|SetProgress (Variables|Default|GetLoading_Ref) _plotgrow_2 "(R=1.000000,G=1.000000,B=1.000000,A=1.000000)" "(R=0.000000,G=1.000000,B=0.109550,A=1.000000)"))
        (:Finished
          (Variables|Default|SetIsResourceComplete? true)
          (Development|PrintString "GrowUp")
          (Variables|Default|SetFood (* (.foodvalue (stale Custom|PlantPlot _returnvalue)) (Variables|Default|GetOutputMultiplier))))))
    (:then_2
      (bind _plotgrow_3 (Timeline|PlantGrowTime Stop) ; Tree
        (:Update
          (Default|SetProgress (Variables|Default|GetLoading_Ref) _plotgrow_3 "(R=1.000000,G=1.000000,B=1.000000,A=1.000000)" "(R=0.274724,G=0.000000,B=1.000000,A=1.000000)"))
        (:Finished
          (Variables|Default|SetFullGrowUpTree true)
          (Default|SetProgress (Variables|Default|GetLoading_Ref) 0.0)
          (Components|Timeline|SetPlayRate (Variables|Default|GetFruitGrowTime) (/ 1.0 (.growtime (stale Custom|PlantPlot _returnvalue))))
          (Timeline|FruitGrowTime Play))))))

(event EventActivateWorkingBuilding
  ;[1 1 1] GetPlotInformation
  (if (Variables|Default|GetHasAlreadyAnItem?)
    (if (Variables|Default|GetIsAPlot?)
      ;;[1 1 1] GrowUpMechanic
      (bind _plotgrow (Timeline|PlotGrowTime Play) ; Plot
        (:Update
          (Default|SetProgress (Variables|Default|GetLoading_Ref) _plotgrow "(R=1.000000,G=1.000000,B=1.000000,A=1.000000)" "(R=0.000000,G=1.000000,B=0.109550,A=1.000000)"))
        (:Finished
          (Variables|Default|SetIsResourceComplete? true)
          (Development|PrintString "GrowUp")
          (Variables|Default|SetFood (* (Variables|Default|GetOutputMultiplier) (.foodvalue (stale Custom|PlantPlot _returnvalue))))))
      (elif (Variables|Default|GetFullGrowUpTree)
        (bind _plotgrow_2 (Timeline|FruitGrowTime Play)
          (:Update
            (Default|SetProgress (Variables|Default|GetLoading_Ref) _plotgrow_2 "(R=1.000000,G=1.000000,B=1.000000,A=1.000000)" "(R=0.000000,G=1.000000,B=0.109550,A=1.000000)"))
          (:Finished
            (Variables|Default|SetIsResourceComplete? true)
            (Development|PrintString "GrowUp")
            (Variables|Default|SetFood (* (.foodvalue (stale Custom|PlantPlot _returnvalue)) (Variables|Default|GetOutputMultiplier)))))
        (else
          (bind _plotgrow_3 (Timeline|PlantGrowTime Play) ; Tree
            (:Update
              (Default|SetProgress (Variables|Default|GetLoading_Ref) _plotgrow_3 "(R=1.000000,G=1.000000,B=1.000000,A=1.000000)" "(R=0.274724,G=0.000000,B=1.000000,A=1.000000)"))
            (:Finished
              (Variables|Default|SetFullGrowUpTree true)
              (Default|SetProgress (Variables|Default|GetLoading_Ref) 0.0)
              (Components|Timeline|SetPlayRate (Variables|Default|GetFruitGrowTime) (/ 1.0 (.growtime (stale Custom|PlantPlot _returnvalue))))
              (Timeline|FruitGrowTime Play))))))))

(fn ConstructionScript
  (|CallParentFunction))

(fn ResourceCollected
  (if (Variables|Default|GetIsAPlot?)
    (if (Variables|Default|GetIsResourceComplete?)
      (Default|UpdateResources (Variables|Default|GetControllerRef) 0.0 0.0 (Variables|Default|GetFood) (Variables|Default|GetWater) 0.0)
      (Variables|Default|SetHasAlreadyAnItem? false)
      (Variables|/Game/Blueprints/UserInterface/DynamicCircle_Widget.DynamicCircle_Widget_C|SetNameText (Variables|Default|GetLoading_Ref) "")
      (Variables|Default|SetIsResourceComplete? false)
      (Default|SetProgress (Variables|Default|GetLoading_Ref) 0.0)
      (Rendering|SetVisibility (Variables|Default|GetResourceLoad) false false)
      (return)
      (else
        _))
    (elif (Variables|Default|GetIsResourceComplete?)
      (CallFunction|ReGrowFruit)
      (Default|UpdateResources (Variables|Default|GetControllerRef) 0.0 0.0 (Variables|Default|GetFood) (Variables|Default|GetWater) 0.0)
      (Variables|Default|SetIsResourceComplete? false)
      (return)
      (else
        _)))
  (Development|PrintString "NeedMoreTime"))

(fn DeletePlot
  (Variables|Default|SetHasAlreadyAnItem? false)
  (Variables|/Game/Blueprints/UserInterface/DynamicCircle_Widget.DynamicCircle_Widget_C|SetNameText (Variables|Default|GetLoading_Ref) "")
  (Variables|Default|SetIsResourceComplete? false))