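; Resource building Blueprint that tracks whether the player character is close to it.
; On BeginPlay it caches the DynamicCircle widget from its ResourceLoad component as LoadingRef.
; Hitbox overlap records the player as inside, sets the character's close-to-resource flag and passes itself as BuildingMasterREF.
; Exit uses actor-level end overlap rather than the Hitbox event, clearing both flags but leaving that reference set.
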(event OnComponentBeginOverlap(Hitbox)
  (params (OverlappedComponent :type Primitive%20Component%20Object%20Reference) (OtherActor :type Actor%20Object%20Reference) (OtherComp :type Primitive%20Component%20Object%20Reference) (OtherBodyIndex :type Integer) (bFromSweep :type Boolean) (SweepResult :type Hit%20Result%20Structure%20%28by%20ref%29))
  (bind (_ascharacter_blueprint _bsuccess) (Utilities|Casting|CastToCharacter_Blueprint OtherActor))
  ;[1 1 1] DetectsWhenPlayerGetsInside
  (if _bsuccess
    (Variables|Default|SetIsPlayerInsideWhenCompleted? true)
    (Variables|/Game/Blueprints/Character/Character_Blueprint.Character_Blueprint_C|SetImCloseToResource? _ascharacter_blueprint true)
    (Variables|/Game/Blueprints/Character/Character_Blueprint.Character_Blueprint_C|SetBuildingMasterREF _ascharacter_blueprint self)))

(event Collision|EventActorEndOverlap
  (params (OtherActor :type Actor%20Object%20Reference))
  (bind (_ascharacter_blueprint _bsuccess) (Utilities|Casting|CastToCharacter_Blueprint OtherActor))
  ;[1 1 1] DetectsWhenPlayerGetsInside
  (if _bsuccess
    (Variables|Default|SetIsPlayerInsideWhenCompleted? false)
    (Variables|/Game/Blueprints/Character/Character_Blueprint.Character_Blueprint_C|SetImCloseToResource? _ascharacter_blueprint false)))

(event Collision|EventActorBeginOverlap
  (params (OtherActor :type Actor%20Object%20Reference))
  (|CallParentFunction OtherActor) ; This node is disabled and will not be called.\nDrag off pins to build functionality.
)

(event EventTick
  (params (DeltaSeconds :type Float%20%28single-precision%29))
  (|CallParentFunction DeltaSeconds) ; This node is disabled and will not be called.\nDrag off pins to build functionality.
)

(event EventBeginPlay
  (|CallParentFunction)
  (Variables|Default|SetLoading_Ref (.AsDynamic%20Circle%20Widget (Utilities|Casting|CastToDynamicCircle_Widget (UserInterface|GetUserWidgetObject (Variables|Default|GetResourceLoad))))))

(fn ConstructionScript
  (|CallParentFunction))