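; Water resource building that produces water on a timed cycle and hands it to the controller's resources when collected.
; WaterFill starts a timeline scaled by SpeedRecolect that drives a progress widget, or, if water is ready, collects it and calls itself to restart.
; The timeline's update and finish logic sits in ActivateWorkingBuilding; finishing marks water ready and multiplies the stored amount by WaterMultiplier.
; DeactivateWorkingBuilding stops the timeline and clears the ready flag.
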(event Custom|WaterFill
  (if (Variables|Default|GetImActive?)
    (if (Variables|Default|GetIsResourceComplete?)
      (CallFunction|RecolectWater)
      (CallFunction|WaterFill)
      (elif (Variables|Default|GetIsBuildingCompleted?)
        (if (not (Variables|Default|GetGettingWater?))
          (Variables|Default|SetGettingWater? true)
          (Variables|/Game/Blueprints/UserInterface/DynamicCircle_Widget.DynamicCircle_Widget_C|SetNameText (Variables|Default|GetLoading_Ref) "Water")
          (Rendering|SetVisibility (Variables|Default|GetResourceLoad) true false)
          (Components|Timeline|SetPlayRate (Variables|Default|GetWaterTimeline) (/ 1.0 (Variables|Default|GetSpeedRecolect)))
          (bind _water (Timeline|WaterTimeline PlayFromStart)
            (:Update
              (Default|SetProgress (Variables|Default|GetLoading_Ref) _water "(R=1.000000,G=1.000000,B=1.000000,A=1.000000)" "(R=0.000000,G=1.000000,B=0.109550,A=1.000000)"))
            (:Finished
              (Variables|Default|SetIsResourceComplete? true)
              (Variables|Default|SetWater (* (Variables|Default|GetWater) (Variables|Default|GetWaterMultiplier)))
              (Development|PrintString "CanBeRecolected"))))))))

(event Custom|RecolectWater
  (Default|UpdateResources (Variables|Default|GetControllerRef) 0.0 0.0 0.0 (Variables|Default|GetWater) 0.0)
  (Default|SetProgress (Variables|Default|GetLoading_Ref) 0.0)
  (Variables|/Game/Blueprints/UserInterface/DynamicCircle_Widget.DynamicCircle_Widget_C|SetNameText (Variables|Default|GetLoading_Ref) "")
  (Variables|Default|SetIsResourceComplete? false)
  (Variables|Default|SetGettingWater? false)
  (Rendering|SetVisibility (Variables|Default|GetResourceLoad) false false))

(event EventBeginPlay
  (|CallParentFunction))

(event Collision|EventActorBeginOverlap
  (params (OtherActor :type Actor%20Object%20Reference))
  (|CallParentFunction OtherActor))

(event EventTick
  (params (DeltaSeconds :type Float%20%28single-precision%29))
  (|CallParentFunction DeltaSeconds) ; This node is disabled and will not be called.\nDrag off pins to build functionality.
)

(event EventActivateWorkingBuilding
  (if (Variables|Default|GetIsBuildingCompleted?)
    (if (Variables|Default|GetGettingWater?)
      (bind _water (Timeline|WaterTimeline Play)
        (:Update
          (Default|SetProgress (Variables|Default|GetLoading_Ref) _water "(R=1.000000,G=1.000000,B=1.000000,A=1.000000)" "(R=0.000000,G=1.000000,B=0.109550,A=1.000000)"))
        (:Finished
          (Variables|Default|SetIsResourceComplete? true)
          (Variables|Default|SetWater (* (Variables|Default|GetWater) (Variables|Default|GetWaterMultiplier)))
          (Development|PrintString "CanBeRecolected"))))))

(event EventDeactivateWorkingBuilding
  (Variables|Default|SetIsResourceComplete? false)
  (bind _water (Timeline|WaterTimeline Stop)
    (:Update
      (Default|SetProgress (Variables|Default|GetLoading_Ref) _water "(R=1.000000,G=1.000000,B=1.000000,A=1.000000)" "(R=0.000000,G=1.000000,B=0.109550,A=1.000000)"))
    (:Finished
      (Variables|Default|SetIsResourceComplete? true)
      (Variables|Default|SetWater (* (Variables|Default|GetWater) (Variables|Default|GetWaterMultiplier)))
      (Development|PrintString "CanBeRecolected"))))

(fn ConstructionScript
  (|CallParentFunction))