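; Capsule Blueprint among the resource buildings, whose own logic rolls how many traits to assign.
; GetRandomTraits draws a random 0–100 integer and compares it to a threshold lowered cumulatively by each TraitMaxChance entry.
; The first threshold met sets NumberOfTraits, with earlier entries giving higher counts and no match giving zero.
; BeginPlay and the construction script only call the parent, and nothing here calls the roll.
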(event EventBeginPlay
  (|CallParentFunction))

(event Collision|EventActorBeginOverlap
  (params (OtherActor :type Actor%20Object%20Reference))
  (|CallParentFunction OtherActor) ; This node is disabled and will not be called.\nDrag off pins to build functionality.
)

(event EventTick
  (params (DeltaSeconds :type Float%20%28single-precision%29))
  (|CallParentFunction DeltaSeconds) ; This node is disabled and will not be called.\nDrag off pins to build functionality.
)

(fn ConstructionScript
  (|CallParentFunction))

(fn GetRandomTraits
  (bind _traitmaxchance (Variables|Default|GetTraitMaxChance))
  (Variables|Default|SetRandom (Math|Random|RandomIntegerinRange 0 100))
  (bind (_array_element _array_index) (Utilities|Array|ForEachLoopwithBreak _traitmaxchance :!label _label)
    (:LoopBody
      (bind _output_get (Variables|Default|SetProbSubtraction (- (Variables|Default|GetProbSubtraction) _array_element)))
      (if (>= (Variables|Default|GetRandom) _output_get)
        (Variables|Default|SetNumberOfTraits (- (Utilities|Array|Length _traitmaxchance) _array_index))
        (goto _label Break)
        (else
          (Variables|Default|SetNumberOfTraits 0))))
    (:Completed
      (return))))