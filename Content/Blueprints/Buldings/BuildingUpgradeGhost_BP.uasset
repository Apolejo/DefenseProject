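; BuildingUpgradeGhost_BP is a placeholder actor that shows the mesh of a building upgrade for a delay, then replaces itself with the building.
; On BeginPlay it sets the ghost mesh and plays a timeline with its rate scaled by the inverse of Delay.
; When the timeline finishes, it spawns BuildingClass at its own transform, passes on ControllerRef, marks the building completed and destroys itself.
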(event Custom|SpawnActor
  (params (SpawnTransform :type Transform) (ControllerRef :type Player%20Game%20Controller%20Object%20Reference))
  (bind _returnvalue (Game|SpawnActorfromClass (Variables|Default|GetBuildingClass) SpawnTransform "AdjustIfPossibleButAlwaysSpawn" 0 ControllerRef 0))
  (Variables|/Game/Blueprints/Buldings/BuildingMaster_BP.BuildingMaster_BP_C|SetIsBuildingCompleted? _returnvalue true)
  (Actor|DestroyActor))

(event EventBeginPlay
  (Components|StaticMesh|SetStaticMesh (Variables|Default|GetUpgradeMeshGhost) (Variables|Default|GetStaticMeshUpgrade))
  (Components|Timeline|SetPlayRate (Variables|Default|GetGhostDelay) (/ 1.0 (Variables|Default|GetDelay)))
  (Timeline|GhostDelay PlayFromStart
    (:Finished
      (CallFunction|SpawnActor (Transformation|GetActorTransform) (Variables|Default|GetControllerRef)))))

(fn ConstructionScript)