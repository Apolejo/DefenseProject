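; Player controller that sets up and triggers building placement through a ghost preview.
; On BeginPlay it enables game-and-UI input and spawns the construction manager and a reusable ghost building, keeping references to both.
; ConstructBuildings spawns the requested building class at the world origin, then resets the ghost and feeds it that actor's display mesh and construction proxy, plus the building class.
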(event EventBeginPlay
  (bind _returnvalue (Math|Transform|MakeTransform "0, 0, 0"))
  (Utilities|FlowControl|Sequence
    (:then_1
      (Input|SetInputModeGameandUI self 0 "DoNotLock" true))
    (:then_2
      (bind _returnvalue_2 (Game|SpawnActorfromClass "/Game/Blueprints/Constructions/ConstructionManager_BP.ConstructionManager_BP_C" _returnvalue "AlwaysSpawn" 0 0))
      (Variables|Default|SetConstructionManagerRef _returnvalue_2))
    (:then_3
      (bind _returnvalue_3 (Game|SpawnActorfromClass "/Game/Blueprints/Buldings/GhostBuilding_BP.GhostBuilding_BP_C" _returnvalue "AlwaysSpawn" 0 self 0))
      (Variables|Default|SetGhostBuildingRef _returnvalue_3))))

(event EventTick
  (params (DeltaSeconds :type Float%20%28single-precision%29)))

(event EventConstructBuildings
  (params (MainBuilding :type Building%20Master%20BP%20Class%20Reference))
  (bind _ghostbuildingref (Variables|Default|GetGhostBuildingRef))
  (bind _returnvalue (Game|SpawnActorfromClass MainBuilding (Math|Transform|MakeTransform "0, 0, 0") "Undefined" 0 self 0))
  (bind _asbuilding_master_bp (Utilities|Casting|CastToBuildingMaster_BPClass MainBuilding))
  (Default|KillGhost _ghostbuildingref)
  (Default|OnSpawn _ghostbuildingref (Variables|/Game/Blueprints/Buldings/BuildingMaster_BP.BuildingMaster_BP_C|GetDisplayMesh _returnvalue) _asbuilding_master_bp (Variables|/Game/Blueprints/Buldings/BuildingMaster_BP.BuildingMaster_BP_C|GetConstructionProxy _returnvalue)))

(fn ConstructionScript)